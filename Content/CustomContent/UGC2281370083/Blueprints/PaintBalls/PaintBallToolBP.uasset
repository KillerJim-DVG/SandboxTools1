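; Paintball tool actor that shoots coloured paintball props into the world on left click.
; The server spawns each PaintBallPropBP from the bullet point transform with the current size and colour, then updates the owning client's tool history so delete works.
; The locally controlled owner initialises once, showing tool assist, loading saved settings and pushing them to the server.
; The settings widget is created on demand, and later setting changes also sync to the server.
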(event Custom|UpdateHistoryOwningClient
  (params (ObjectToAttach :type Actor%20Object%20Reference))
  ;[1 1 1] Update the history (to reflect last selection as most recent)
  (Class|KJModToolProxy|AddHistoryEntry (Utilities|Struct|MakeKJModToolHistoryItem ObjectToAttach "paintball" "Paintball" "DeleteItem")))

(event EventBeginPlay
  ;[0.9593 1 0.1335] BEGIN PLAY EVENT
  (Networking|SwitchHasAuthority
    (:Authority
      ;;[1 1 1] Listen server?
      (if (not (Networking|IsDedicatedServer))
        ;;[1 1 1] If local controlled; init once..
        (Utilities|IsLocallyControlled :!label _label
          (:LocalControl
            (CallFunction|NotifyOwnerOfInstantiation)
            (if (not (Variables|Initialisation|GetInitialised))
              (Variables|Initialisation|SetInitialised true)
              ;;[1 1 1] Reload settings
              (CallFunction|CreateandShowToolsAssistInformation)
              (CallFunction|InitSettings))))))
    (:Remote
      (goto _label))))

(event Custom|SpawnPaintballServer
  (params (SpawnTransform :type Transform))
  (bind _settings (Variables|ToolSetting|GetSettings))
  (bind (_size _colour) (Utilities|Struct|BreakPaintBallToolActorSettings _settings))
  ;[1 1 1] Spawn projectile (replicated to others)
  (bind _returnvalue (Game|SpawnActorfromClass "/Game/CustomContent/UGC2281370083/Blueprints/PaintBalls/Prop/PaintBallPropBP.PaintBallPropBP_C" SpawnTransform "AlwaysSpawn" (Components|GetOwner self) _size _colour 0))
  (CallFunction|UpdateHistoryOwningClient _returnvalue) ; Runs on tool owner, allows delete to work
)

(event EventToolProxyPrimaryMouseClick
  (params (pressed :type Boolean))
  ;[1 1 1] Left mouse? Spawn projectile on server
  (if pressed ; Pressed?
    (CallFunction|SpawnPaintballServer (Transformation|GetWorldTransform (Variables|Default|GetBulletPoint)))))

(event Custom|Setting_SetColor
  (params (Color :type Linear%20Color%20Structure))
  ;[1 1 1] Settings (from widgets and onload)
  (Utilities|Struct|SetmembersinPaintBallToolActorSettings (Variables|ToolSetting|GetSettings) Color)
  ;[1 1 1] Update server
  (if (Variables|ToolSetting|GetbServerSettingsInited)
    (CallFunction|SetPaintBallSettingsOwningClient (Variables|ToolSetting|GetSettings))))

(event Custom|Setting_SetSize
  (params (Value :type Float%20%28single-precision%29))
  ;[1 1 1] Settings (from widgets and onload)
  (Utilities|Struct|SetmembersinPaintBallToolActorSettings (Variables|ToolSetting|GetSettings) Value)
  ;[1 1 1] Update server
  (if (Variables|ToolSetting|GetbServerSettingsInited)
    (CallFunction|SetPaintBallSettingsOwningClient (Variables|ToolSetting|GetSettings))))

(event Custom|SetPaintBallSettingsOwningClient
  (params (Settings :type Paint%20Ball%20Tool%20Actor%20Settings%20Structure))
  ;[1 1 1] Make sure the settings reach the server-side; this is where things are spawned
  (CallFunction|SetPaintBallSettingsServer Settings))

(event Custom|SetPaintBallSettingsServer
  (params (Settings :type Paint%20Ball%20Tool%20Actor%20Settings%20Structure))
  ;[1 1 1] Make sure the settings reach the server-side; this is where things are spawned
  (Variables|ToolSetting|SetSettings Settings))

(event Custom|InitSettings
  ;[1 1 1] Init / Load previous settings
  (bind _returnvalue (Class|KJModToolProxy|LoadToolSettings "PaintballToolSettings"))
  (Utilities|IsValid _returnvalue ; No save? use defaults
    (:Is%20Valid
      (bind _aspaint_ball_tool_save_game_bp (Utilities|Casting|CastToPaintBallToolSaveGameBP _returnvalue))
      (Utilities|FlowControl|Sequence
        (:then_0
          ;[1 1 1] Local Initial settings
          (Utilities|FlowControl|Sequence
            (:then_0
              (CallFunction|SettingSetSize (Variables|/Game/CustomContent/UGC2281370083/Blueprints/PaintBalls/PaintBallToolSaveGameBP.PaintBallToolSaveGameBP_C|GetSize _aspaint_ball_tool_save_game_bp)))
            (:then_1
              (CallFunction|SettingSetColor (Variables|/Game/CustomContent/UGC2281370083/Blueprints/PaintBalls/PaintBallToolSaveGameBP.PaintBallToolSaveGameBP_C|GetColor _aspaint_ball_tool_save_game_bp)))))
        (:then_1
          ;[1 1 1] Init settings server
          (CallFunction|SetPaintBallSettingsOwningClient (Variables|ToolSetting|GetSettings) :!label _label)
          (Variables|ToolSetting|SetbServerSettingsInited true))))
    (:Is%20Not%20Valid
      (goto _label))))

(fn ConstructionScript)

(fn CreateandShowToolsAssistInformation
  (Class|KJModToolProxy|ShowToolAssistUI)
  (Class|KJModToolProxy|SetToolAssistTitle "Paintball" "Shoot paintballs to colour the world")
  (Class|KJModToolProxy|ClearToolAssistFunctions)
  (bind _returnvalue (Class|KJModToolProxy|CreateToolAssistFunction "Shoot a paintball"))
  (Class|KJModToolProxy|SetToolAssistFunctionPrimaryDetails _returnvalue "LeftMouse"))

(fn ToolProxyGetToolSettingPanel
  (Utilities|IsValid (Variables|ToolSetting|GetToolSettingsWidget)
    (:Is%20Valid
      _)
    (:Is%20Not%20Valid
      (bind _returnvalue (UserInterface|CreateWidget "/Game/CustomContent/UGC2281370083/Blueprints/PaintBalls/Settings/PaintBallToolSettingsWidgetBP.PaintBallToolSettingsWidgetBP_C" (Game|GetPlayerController 0) self))
      (Default|CreatedEvent _returnvalue)
      (Variables|ToolSetting|SetToolSettingsWidget _returnvalue)))
  (return (Variables|ToolSetting|GetToolSettingsWidget)))