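; Physics paintball prop that leaves a colored splat decal on the first non-paintball component it hits.
; The server records the impact in a replicated struct and freezes the ball, keeping the actor alive for late joiners.
; Its RepNotify waits briefly for the hit component to replicate, then clients hide the ball and spawn the decal, plus a particle splash only for fresh impacts.
; Destroying the actor removes the decal.
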(event Custom|SplatImpactDecal
  (bind _replicationimpactstruct (Variables|Default|GetReplicationImpactStruct))
  (bind (_attachcomponent _size _location _rotation _color) (Utilities|Struct|BreakPaintBallRepStruct _replicationimpactstruct))
  ;[0.2179 1 0] Remotely visualise splat
  ;;[1 0.5954 0.08993] On join a new users will get this actor; but what it's attached to (if it's spawned in world, and not in the level) may not be replicated into the world (i.e. this splat is replicated first, then what it's attached to appears a few milliseconds later)
  (Variables|Default|SetTimeout 10)
  (Utilities|IsValid _attachcomponent :!label _label ; Wait for replication (on join, hopefully it's here already)
    (:Is%20Valid
      (Utilities|HandleClientServerLogic
        (:ClientLogic
          (bind _returnvalue (Class|GameplayStatics|SpawnDecalAttached "/Game/CustomContent/UGC2281370083/Blueprints/PaintBalls/Prop/SplatMaterial.SplatMaterial" (Math|Vector|MakeVector 15.0 _size _size) _attachcomponent "None" _location _rotation "KeepWorldPosition" 0.0))
          (bind _output_get (Variables|Default|SetDecalActor _returnvalue))
          (bind _returnvalue_2 (Rendering|Material|CreateDynamicMaterialInstance _output_get :!class /Script/Engine.DecalComponent))
          (Rendering|Material|SetScalarParameterValue _returnvalue_2 "Frame" (Math|Conversions|ToFloat(Integer) (Math|Random|RandomIntegerinRange 0 15)) :!class /Script/Engine.MaterialInstanceDynamic)
          (Rendering|Material|SetVectorParameterValue _returnvalue_2 "Color" _color :!class /Script/Engine.MaterialInstanceDynamic)
          ;;[1 1 1] If too much time has passed; no point in replicating the splash
          (if (Variables|Default|GetDisableReplicatedParticleSplash)
            _
            (else
              (bind _returnvalue_3 (Effects|SpawnEmitteratLocation "/Game/CustomContent/UGC2281370083/Blueprints/PaintBalls/Particles/PaintballImpactParticle.PaintballImpactParticle" _location _rotation (/ (Math|Conversions|ToVector(Float) _size) 5e+01)))
              (Effects|Components|ParticleSystem|SetColorParameter _returnvalue_3 "Color" _color)))
          ;;[1 1 1] On impact, hide the sphere and disable interactions so it's effectively "quiet"
          (Rendering|SetVisibility (Variables|Default|GetSphere) false false)
          (Physics|SetSimulatePhysics (Variables|Default|GetSphere) false)
          (Collision|SetCollisionEnabled (Variables|Default|GetSphere) "NoCollision"))))
    (:Is%20Not%20Valid
      (Utilities|FlowControl|Delay 0.1)
      (bind _result (Math|Integer|DecrementInt (Variables|Default|GetTimeout))
        (:%20%20
          (if (not (< _result 0))
            (goto _label)))))))

(event EventDestroyed
  ;[1 0.01528 0] When destroyed (like deleted by the user) - destroy the decal, the particles are long gone..
  (Utilities|IsValid (Variables|Default|GetDecalActor)
    (:Is%20Valid
      (Components|DestroyComponent (Variables|Default|GetDecalActor)))))

(event EventBeginPlay
  ;[0.2555 1 0] EVENT PLAY - Make sure the  sphere is the correct color
  (bind _returnvalue (Rendering|Material|CreateDynamicMaterialInstance (Variables|Default|GetSphere) 0 "/Game/CustomContent/UGC2281370083/Blueprints/PaintBalls/Prop/PaintballMaterial.PaintballMaterial" "None" :!class /Script/Engine.PrimitiveComponent))
  (Rendering|Material|SetVectorParameterValue _returnvalue "Color" (Variables|Default|GetColor) :!class /Script/Engine.MaterialInstanceDynamic))

(event Collision|EventHit
  (params (MyComp :type Primitive%20Component%20Object%20Reference) (Other :type Actor%20Object%20Reference) (OtherComp :type Primitive%20Component%20Object%20Reference) (bSelfMoved :type Boolean) (HitLocation :type Vector :default "0, 0, 0") (HitNormal :type Vector :default "0, 0, 0") (NormalImpulse :type Vector :default "0, 0, 0") (Hit :type Hit%20Result%20Structure%20%28by%20ref%29))
  ;[1 1 1] Event Hit - If the impact has not occured, and it's not another paintball, then on the server handle the impact, spawning a decal on remote machines
  (if (not (Variables|Default|GetImpactOccured))
    (if (not (Components|ComponentHasTag OtherComp "Paintball"))
      (Utilities|HandleClientServerLogic
        (:ServerLogic
          (Variables|Default|SetImpactOccured true)
          (Variables|Default|SetReplicationImpactStruct (Utilities|Struct|MakePaintBallRepStruct OtherComp (Math|Random|RandomFloatinRange (* (Variables|Default|GetSize) 2.5) (* (Variables|Default|GetSize) 6.0)) HitLocation (Math|Conversions|RotationFromXVector HitNormal) (Variables|Default|GetColor)))
          ;;[1 1 1] Stop all interactions (as this actor freezes in place, living on the RepNotify clients joining of the splat)
          (Physics|SetSimulatePhysics (Variables|Default|GetSphere) false)
          (Collision|SetCollisionEnabled (Variables|Default|GetSphere) "NoCollision")
          ;;[1 1 1] After 200ms no point in anyone showing the splash (i.e. late joiners)
          (Utilities|FlowControl|Delay 0.2)
          (Variables|Default|SetDisableReplicatedParticleSplash true))))))

(fn ConstructionScript)

(fn OnRepReplicationImpactStruct
  ;[1 1 1] called when this actor is on replicated spawn (or late joining long after this hit some object)
  (CallFunction|SplatImpactDecal))