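; Player tool that places configurable, triggerable physics wheels on traced surfaces.
; A client camera trace positions a ghost wheel along the surface normal and sends the hit target to the server.
; Left-click spawns a wheel that the server attaches and registers for triggers; right-click reverses the last one.
; Saved and widget settings sync to the server, type changes respawn the ghost, and OnRep records placed wheels in undo history.
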(event Custom|AdjustGhostWheelSettings
  (params (Settings :type Wheels%20Tool%20Actor%20Settings%20Structure))
  ;[1 1 1] GHOST WHEEL - Settings
  (Utilities|IsValid (Variables|Ghosting|GetGhostWheel)
    (:Is%20Valid
      (Default|SetGhostWheelSettingsOwningClient (Variables|Ghosting|GetGhostWheel) Settings))))

(event Custom|UpdateHistoryOwningClient
  (params (ObjectToAttach :type Actor%20Object%20Reference))
  ;[1 1 1] Update the history (to reflect last selection as most recent)
  (Class|KJModToolProxy|AddHistoryEntry (Utilities|Struct|MakeKJModToolHistoryItem ObjectToAttach "Removing wheel" "Wheel" "DeleteItem")))

(event Custom|SetWheelInformationOwningClient
  (params (Location :type Vector) (Visible :type Boolean) (TargetActor :type Actor%20Object%20Reference) (TargetComponent :type Primitive%20Component%20Object%20Reference) (Rotation :type Rotator))
  (bind _ghostwheel (Variables|Ghosting|GetGhostWheel))
  ;[1 1 1] Update ghost wheel position and settings information (local and remote)
  (CallFunction|SetWheelInformationServer Location Visible TargetActor TargetComponent Rotation)
  (Utilities|IsValid _ghostwheel ; may not be replicated yet
    (:Is%20Valid
      (Transformation|SetActorLocation _ghostwheel Location false true)
      (Transformation|SetActorRotation _ghostwheel Rotation true)
      (Rendering|SetActorHiddenInGame _ghostwheel (not Visible)))))

(event Custom|SetWheelInformationServer
  (params (Location :type Vector) (Visible :type Boolean) (TargetActor :type Actor%20Object%20Reference) (TargetComponent :type Primitive%20Component%20Object%20Reference) (Rotation :type Rotator))
  (bind _ghostwheel (Variables|Ghosting|GetGhostWheel))
  ;[1 1 1] Update ghost wheel position and settings information (local and remote)
  (Utilities|Struct|SetmembersinWheelsToolActorSettings (Variables|ToolSetting|GetSettings) TargetActor TargetComponent)
  (Utilities|IsValid _ghostwheel ; Is null when switching lamp's
    (:Is%20Valid
      (Transformation|SetActorLocation _ghostwheel Location false true)
      (Transformation|SetActorRotation _ghostwheel Rotation true)
      (Rendering|SetActorHiddenInGame _ghostwheel (not Visible)))))

(event EventDestroyed
  (bind _ghostwheel (Variables|Ghosting|GetGhostWheel))
  ;[1 1 1] DESTROYED - remove ghost wheel from server
  (Utilities|IsValid _ghostwheel
    (:Is%20Valid
      (Actor|DestroyActor _ghostwheel))))

(event EventBeginPlay
  ;[0.9593 1 0.1335] BEGIN PLAY EVENT
  (Utilities|HandleClientServerLogic
    (:ClientLogic
      ;;[1 1 1] If local controlled; init once..
      (Utilities|IsLocallyControlled
        (:LocalControl
          (CallFunction|NotifyOwnerOfInstantiation)
          (if (not (Variables|Initialisation|GetInitialised))
            (Variables|Initialisation|SetInitialised true)
            ;;[1 1 1] Reload settings
            (CallFunction|CreateandShowToolsAssistInformation)
            (CallFunction|InitSettings)
            (CallFunction|InitTriggerSettings)
            ;;[1 1 1] Create ghost wheel
            (CallFunction|CreateGhostWheel (Utilities|Struct|BreakWheelsToolActorSettings (Variables|ToolSetting|GetSettings)))))))))

(event EventTick
  (params (DeltaSeconds :type Float%20%28single-precision%29))
  ;[1 1 1] EVENT TICK
  (|CallParentFunction DeltaSeconds)
  (Utilities|IsLocallyControlled
    (:LocalControl
      (Utilities|HandleClientServerLogic
        (:ClientLogic
          ;;[1 1 1] Handle MOUSE SELECTION POINT
          (bind _returnvalue (Class|KJModToolProxy|GetPawnCameraComponent))
          (bind (_outhit _returnvalue_2) (Collision|LineTraceByChannel (Transformation|GetWorldLocation _returnvalue) (+ (Transformation|GetWorldLocation _returnvalue) (* (Math|Vector|GetForwardVector _returnvalue) 3.5e+03)) "TraceTypeQuery1" true (Utilities|Array|MakeArray (Game|Player|GetPlayerPawn 0)) "None"))
          (if _returnvalue_2
            (Utilities|IsValid (.HitActor (Collision|BreakHitResult _outhit))
              (:Is%20Valid
                (Utilities|IsValid (Variables|Ghosting|GetGhostWheel) ; May not be replicated from server (yet)
                  (:Is%20Valid
                    (bind _rotation (Utilities|BuildRotationfromImpactNormal (.ImpactPoint (Collision|BreakHitResult _outhit)) (.ImpactNormal (Collision|BreakHitResult _outhit)))
                      (:Out
                        (bind _output_get (Variables|Ghosting|SetGhostWheelLocation (- (.Location (Collision|BreakHitResult _outhit)) (* (Math|Vector|GetForwardVector _rotation) (Math|Float|MakeLiteralFloat (Variables|/Game/CustomContent/UGC2281370083/Blueprints/Wheels/Props/WheelsBasePropBP.WheelsBasePropBP_C|GetCustomWheelOffset (Variables|Ghosting|GetGhostWheel)))))))
                        (Variables|Ghosting|SetGhostWheelRotation _rotation)
                        (CallFunction|SetWheelInformationOwningClient _output_get true (.HitActor (Collision|BreakHitResult _outhit)) (.HitComponent (Collision|BreakHitResult _outhit)) (Variables|Ghosting|GetGhostWheelRotation))
                        (Variables|Ghosting|SetGhostWheeltVisible true))))
                  (:Is%20Not%20Valid
                    (CallFunction|SetWheelInformationOwningClient "0, 0, 0" false 0 0 "0, 0, 0" :!label _label)
                    (Variables|Ghosting|SetGhostWheeltVisible false))))
              (:Is%20Not%20Valid
                (goto _label)))
            (else
              (goto _label))))))))

(event Custom|ServerReleaseWheel
  (params (WheelToRelease :type Wheels%20Base%20Prop%20BP%20Object%20Reference))
  ;[1 1 1] SERVER - Release Wheel (called when spawning the actual wheel)
  (Default|SetWheelAttachedActor WheelToRelease (Variables|ToolSetting|GetSettings))
  (Class|KJModToolProxy|RegisterTriggerActor WheelToRelease)
  (Class|KJModToolProxy|SetTrigger WheelToRelease (Variables|Default|GetTriggerable) (Variables|Default|GetTriggerType) (Variables|Default|GetTriggerKey) (Variables|Default|GetTriggerEventName)))

(event EventToolProxyItemSpawned
  (params (spawnedActor :type Actor%20Object%20Reference))
  ;[1 1 1] (interface) Item Spawned - From Pawn
  (bind _aswheels_base_prop_bp (Utilities|Casting|CastToWheelsBasePropBP spawnedActor)
    (:then
      (Utilities|IsValid (Variables|Ghosting|GetGhostWheel) ; First time? it's our "ghost" wheel
        (:Is%20Valid
          (bind _output_get (Variables|Spawning|SetSpawnedWheelActor _aswheels_base_prop_bp))
          (CallFunction|ServerReleaseWheel _output_get) ; A real wheel has been spawned
        )
        (:Is%20Not%20Valid
          (Variables|Ghosting|SetGhostWheel _aswheels_base_prop_bp))))
    (:CastFailed
      (|CallParentFunction spawnedActor) ; Probably a Q menu spawning; let parent deal with it
    )))

(event Custom|SwitchDirection
  ;[1 1 1] LEFT/RIGHT MOUSE - Drop or freeze if anything on tool
  ;;[1 1 1] Left - Attempt Grab or Release any object
  (Default|ChangeDirectionServer (Variables|Spawning|GetSpawnedWheelActor)))

(event EventToolProxySecondaryMouseClick
  (params (pressed :type Boolean))
  ;[1 1 1] LEFT/RIGHT MOUSE - Drop or freeze if anything on tool
  ;;[1 1 1] Left - Attempt Grab or Release any object
  (if pressed ; Pressed?
    (Utilities|IsValid (Variables|Spawning|GetSpawnedWheelActor)
      (:Is%20Valid
        (CallFunction|SwitchDirection)))))

(event EventToolProxyPrimaryMouseClick
  (params (pressed :type Boolean))
  ;[1 1 1] LEFT/RIGHT MOUSE - Drop or freeze if anything on tool
  ;;[1 1 1] Left - Attempt Grab or Release any object
  (if pressed ; Pressed?
    (Utilities|IsValid (Variables|Ghosting|GetGhostWheel)
      (:Is%20Valid
        (if (Variables|Ghosting|GetGhostWheeltVisible)
          (if (<= (Variables|Default|GetRespawnDelayTimeout) 0.0)
            (Class|KJModToolProxy|SpawnItem (Utilities|Struct|BreakWheelsToolActorSettings (Variables|ToolSetting|GetSettings)) (Variables|Ghosting|GetGhostWheelLocation) (Variables|Ghosting|GetGhostWheelRotation) "1.000000,1.000000,1.000000")
            (Variables|Default|SetRespawnDelayTimeout 0.5)))))))

(event Custom|Setting_ForceLimit
  (params (Value :type Float%20%28single-precision%29))
  ;[1 1 1] LOAD / REALISE TOOL SPECIFIC SETTINGS
  ;;[1 1 1] Settings (from widgets and onload)
  (bind _structout (Utilities|Struct|SetmembersinWheelsToolActorSettings (Variables|ToolSetting|GetSettings) Value))
  (CallFunction|AdjustGhostWheelSettings _structout)
  ;;[1 1 1] Update server
  (if (Variables|ToolSetting|GetbServerSettingsInited)
    (CallFunction|SetShweelSettingsOwningClient (Variables|ToolSetting|GetSettings))))

(event Custom|TriggerWidgetSettingsChanged
  ;[1 1 1] TRIGGER SETTINGS CHANGED - Call via dispatched event on trigger widget
  (CallFunction|InitTriggerSettings))

(event Custom|SetWheelActorBP
  (params (Type :type String))
  ;[1 1 1] LOAD / REALISE TOOL SPECIFIC SETTINGS
  ;;[1 1 1] TYPE CHANGE - If type is changed destroy old "ghost" type, and create a new one with the correct actor BP
  (CallFunction|RemovePreviousWheelActorBP (Variables|Ghosting|GetGhostWheel) Type))

(event Custom|InitSettings
  ;[1 1 1] LOAD / REALISE TOOL SPECIFIC SETTINGS
  ;;[1 1 1] Init / Load previous settings
  (bind _returnvalue (Class|KJModToolProxy|LoadToolSettings "Wheels"))
  (Utilities|IsValid _returnvalue ; No save? use defaults
    (:Is%20Valid
      (bind _aswheels_tool_save_game_bp (Utilities|Casting|CastToWheelsToolSaveGameBP _returnvalue))
      (Utilities|FlowControl|Sequence
        (:then_0
          ;;[1 1 1] Local Initial settings
          (Utilities|FlowControl|Sequence
            (:then_0
              (CallFunction|SettingSetTorque (Variables|/Game/CustomContent/UGC2281370083/Blueprints/Wheels/WheelsToolSaveGameBP.WheelsToolSaveGameBP_C|GetTorque _aswheels_tool_save_game_bp)))
            (:then_1
              (CallFunction|SettingForceLimit (Variables|/Game/CustomContent/UGC2281370083/Blueprints/Wheels/WheelsToolSaveGameBP.WheelsToolSaveGameBP_C|GetForceLimit _aswheels_tool_save_game_bp)))
            (:then_2
              (CallFunction|SettingSetType (Variables|/Game/CustomContent/UGC2281370083/Blueprints/Wheels/WheelsToolSaveGameBP.WheelsToolSaveGameBP_C|GetType _aswheels_tool_save_game_bp)))
            (:then_3
              (CallFunction|SettingNoCollision (Variables|/Game/CustomContent/UGC2281370083/Blueprints/Wheels/WheelsToolSaveGameBP.WheelsToolSaveGameBP_C|GetbDisableCollision _aswheels_tool_save_game_bp)))
            (:then_4
              (CallFunction|SettingFriction (Variables|/Game/CustomContent/UGC2281370083/Blueprints/Wheels/WheelsToolSaveGameBP.WheelsToolSaveGameBP_C|GetFriction _aswheels_tool_save_game_bp)))))
        (:then_1
          ;;[1 1 1] Init settings server
          (CallFunction|SetShweelSettingsOwningClient (Variables|ToolSetting|GetSettings) :!label _label)
          (Variables|ToolSetting|SetbServerSettingsInited true))))
    (:Is%20Not%20Valid
      (goto _label))))

(event Custom|Setting_Friction
  (params (Value :type Float%20%28single-precision%29))
  ;[1 1 1] LOAD / REALISE TOOL SPECIFIC SETTINGS
  ;;[1 1 1] Settings (from widgets and onload)
  (bind _structout (Utilities|Struct|SetmembersinWheelsToolActorSettings (Variables|ToolSetting|GetSettings) Value))
  (CallFunction|AdjustGhostWheelSettings _structout)
  ;;[1 1 1] Update server
  (if (Variables|ToolSetting|GetbServerSettingsInited)
    (CallFunction|SetShweelSettingsOwningClient (Variables|ToolSetting|GetSettings))))

(event Custom|Setting_SetTorque
  (params (Value :type Float%20%28single-precision%29))
  ;[1 1 1] LOAD / REALISE TOOL SPECIFIC SETTINGS
  ;;[1 1 1] Settings (from widgets and onload)
  (bind _structout (Utilities|Struct|SetmembersinWheelsToolActorSettings (Variables|ToolSetting|GetSettings) Value))
  (CallFunction|AdjustGhostWheelSettings _structout)
  ;;[1 1 1] Update server
  (if (Variables|ToolSetting|GetbServerSettingsInited)
    (CallFunction|SetShweelSettingsOwningClient (Variables|ToolSetting|GetSettings))))

(event Custom|RemovePreviousWheelActorBP
  (params (Actor :type Actor%20Object%20Reference) (Type :type String))
  ;[1 1 1] LOAD / REALISE TOOL SPECIFIC SETTINGS
  ;;[1 1 1] TYPE CHANGE - If type is changed destroy old "ghost" type, and create a new one with the correct actor BP
  (Utilities|IsValid Actor
    (:Is%20Valid
      (Actor|DestroyActor Actor)
      (Variables|Ghosting|SetGhostWheel 0)
      (Utilities|FlowControl|Delay 0.25)
      (CallFunction|ReInitWheelActor Type))))

(event Custom|Setting_NoCollision
  (params (DisableCollision :type Boolean))
  ;[1 1 1] LOAD / REALISE TOOL SPECIFIC SETTINGS
  ;;[1 1 1] Settings (from widgets and onload)
  (bind _structout (Utilities|Struct|SetmembersinWheelsToolActorSettings (Variables|ToolSetting|GetSettings) DisableCollision))
  (CallFunction|AdjustGhostWheelSettings _structout))

(event Custom|SetShweelSettingsOwningClient
  (params (Settings :type Wheels%20Tool%20Actor%20Settings%20Structure))
  ;[1 1 1] LOAD / REALISE TOOL SPECIFIC SETTINGS
  ;;[1 1 1] Replicate changes (and visualise mesh)
  (CallFunction|SetWheelSettingsServer Settings))

(event Custom|Setting_SetType
  (params (Type :type String))
  ;[1 1 1] LOAD / REALISE TOOL SPECIFIC SETTINGS
  ;;[1 1 1] Settings (from widgets and onload)
  (if (Utilities|Enum|NotEqual(Enum) Type (.Type (Utilities|Struct|BreakWheelsToolActorSettings (Variables|ToolSetting|GetSettings)))) ; Did they change the visualisation?
    (CallFunction|SetWheelActorBP Type))
  (Utilities|Struct|SetmembersinWheelsToolActorSettings (Variables|ToolSetting|GetSettings) Type)
  ;;[1 1 1] Update server
  (if (Variables|ToolSetting|GetbServerSettingsInited)
    (CallFunction|SetShweelSettingsOwningClient (Variables|ToolSetting|GetSettings))))

(event Custom|SetWheelSettingsServer
  (params (Settings :type Wheels%20Tool%20Actor%20Settings%20Structure))
  ;[1 1 1] LOAD / REALISE TOOL SPECIFIC SETTINGS
  ;;[1 1 1] Replicate changes (and visualise mesh)
  (Variables|ToolSetting|SetSettings Settings))

(event Custom|ReInitWheelActor
  (params (Type :type String))
  ;[1 1 1] LOAD / REALISE TOOL SPECIFIC SETTINGS
  ;;[1 1 1] TYPE CHANGE - If type is changed destroy old "ghost" type, and create a new one with the correct actor BP
  (CallFunction|CreateGhostWheel Type))

(event Custom|RealiseSettings
  (params (Triggerable :type Boolean) (Selection :type Integer) (TriggerKey :type Key%20Structure :default "None") (TriggerEventName :type String))
  ;[1 1 1] SERVER LOAD - These settings are used server side
  (Utilities|FlowControl|Sequence
    (:then_0
      (Variables|Default|SetTriggerable Triggerable))
    (:then_1
      (switch int Selection
        (:0
          (Variables|Default|SetTriggerType "KeyHeldTrigger"))
        (:1
          (Variables|Default|SetTriggerType "KeyPressToggle"))
        (:2
          (Variables|Default|SetTriggerType "NamedEventToggleTrigger"))))
    (:then_2
      (Variables|Default|SetTriggerKey TriggerKey))
    (:then_3
      (Variables|Default|SetTriggerEventName TriggerEventName))))

(event Custom|InitTriggerSettings
  ;[1 1 1] LOAD BASE TRIGGER SETTINGS - Grab the base settings and transfer to server (as it spawns the wheel and needs them there)
  (bind _returnvalue (Class|KJModToolProxy|LoadToolSettings "WheelsBaseSettings"))
  (Utilities|IsValid _returnvalue
    (:Is%20Valid
      (bind _asbase_tool_save_game_bp (Utilities|Casting|CastToBaseToolSaveGameBP _returnvalue))
      (CallFunction|RealiseSettings (Variables|/Game/CustomContent/UGC2281370083/Blueprints/BaseToolSaveGameBP.BaseToolSaveGameBP_C|GetTriggerable _asbase_tool_save_game_bp) (Variables|/Game/CustomContent/UGC2281370083/Blueprints/BaseToolSaveGameBP.BaseToolSaveGameBP_C|GetTriggerType _asbase_tool_save_game_bp) (Variables|/Game/CustomContent/UGC2281370083/Blueprints/BaseToolSaveGameBP.BaseToolSaveGameBP_C|GetTriggerKey _asbase_tool_save_game_bp) (Variables|/Game/CustomContent/UGC2281370083/Blueprints/BaseToolSaveGameBP.BaseToolSaveGameBP_C|GetTriggerEventName _asbase_tool_save_game_bp)))))

(fn ConstructionScript)

(fn CreateandShowToolsAssistInformation
  (Class|KJModToolProxy|ShowToolAssistUI)
  (Class|KJModToolProxy|SetToolAssistTitle "Wheels" "A physics based wheel that can be configured")
  (Class|KJModToolProxy|ClearToolAssistFunctions)
  (Utilities|FlowControl|Sequence
    (:then_0
      (bind _returnvalue (Class|KJModToolProxy|CreateToolAssistFunction "Add wheel at required point"))
      (Class|KJModToolProxy|SetToolAssistFunctionPrimaryDetails _returnvalue "LeftMouse"))
    (:then_1
      (bind _returnvalue_2 (Class|KJModToolProxy|CreateToolAssistFunction "Switch direction"))
      (Class|KJModToolProxy|SetToolAssistFunctionPrimaryDetails _returnvalue_2 "RightMouse"))))

(fn CreateGhostWheel
  (params (AssetPath :type String))
  (bind _returnvalue (Game|GetPlayerCameraManager 0))
  (Class|KJModToolProxy|SpawnItem AssetPath (+ (Transformation|GetActorLocation _returnvalue) (* (Transformation|GetActorForwardVector _returnvalue) 5e+02)) "0, 0, 0" "1.000000,1.000000,1.000000"))

(fn ToolProxyGetToolSettingPanel
  (Utilities|IsValid (Variables|ToolSetting|GetToolSettingsWidget)
    (:Is%20Valid
      _)
    (:Is%20Not%20Valid
      (bind _returnvalue (UserInterface|CreateWidget "/Game/CustomContent/UGC2281370083/Blueprints/Wheels/Settings/WheelsToolSettingsWidgetBP.WheelsToolSettingsWidgetBP_C" (Game|GetPlayerController 0) self))
      (Default|CreatedEvent _returnvalue)
      (bind _output_get (Variables|ToolSetting|SetToolSettingsWidget _returnvalue))
      ;[1 1 1] We want to listen to changes from the trigger widget part
      (EventDispatchers|BindEventtoTriggerWidgetUpdated (Variables|/Game/CustomContent/UGC2281370083/Blueprints/Wheels/Settings/WheelsToolSettingsWidgetBP.WheelsToolSettingsWidgetBP_C|GetBaseTriggerWidgetBP _output_get) (EventDispatchers|CreateEvent :!event Custom|TriggerWidgetSettingsChanged))))
  (return (Variables|ToolSetting|GetToolSettingsWidget)))

(fn OnRepSpawnedWheelActor
  (bind _spawnedwheelactor (Variables|Spawning|GetSpawnedWheelActor))
  ;[1 1 1] If we're the owner then record the Wheels creation in our history (for delete)
  (Utilities|IsLocallyControlled
    (:LocalControl
      (Utilities|IsValid _spawnedwheelactor
        (:Is%20Valid
          (CallFunction|UpdateHistoryOwningClient _spawnedwheelactor))))))