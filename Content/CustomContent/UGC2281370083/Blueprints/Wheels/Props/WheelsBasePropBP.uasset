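; Base Blueprint for a wheel prop that bolts onto another physics object and drives it.
; A multicast attach event joins the simulated wheel via a physics constraint; a server timer destroys it if its parent vanishes.
; While active and grounded by a throttled line trace, Tick fakes torque by pushing the connected body at the wheel's location.
; Trigger events toggle drive; direction changes flip torque and respawn an indicator actor.
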(event Custom|SetWheelAttachedActor
  (params (Settings :type Wheels%20Tool%20Actor%20Settings%20Structure))
  ;[1 1 1] SERVER - Attach to actor (spawn physical constraint)
  (CallFunction|SetWheelAttachment Settings))

(event Custom|ChangeDirectionServer
  ;[1 1 1] CHANGE DIRECTION - Server
  (Utilities|IsValid (Variables|Default|GetWheelDirectionActor)
    (:Is%20Valid
      (Actor|DestroyActor (Variables|Default|GetWheelDirectionActor)))
    (:Is%20Not%20Valid
      _))
  (bind _output_get (Variables|Default|SetForwardDirection (not (Variables|Default|GetForwardDirection))))
  (CallFunction|ShowDirectionIndicator _output_get)
  (CallFunction|ChangeDirectionMulticast))

(event Custom|SetGhostWheelSettingsOwningClient
  (params (Settings :type Wheels%20Tool%20Actor%20Settings%20Structure))
  ;[1 1 1] GHOST WHEEL - Updating any parameters (run-time) - Technically a wheel only changes type at run-time but we keep it as example code
  (Utilities|FlowControl|RetriggerableDelay 0.1) ; Stop flooding of network on lots of changes.. wait 100ms
)

(event Custom|EnsureConnectionIsValid
  ;[1 1 1] If conected to something, make sure it exists or delete ourselves
  (Networking|SwitchHasAuthority
    (:Authority
      (Utilities|Time|SetTimerbyEvent (delegate Custom|ConnectionCheck) 0.1 true))))

(event Custom|ConnectionCheck
  ;[1 1 1] If conected to something, make sure it exists or delete ourselves
  (Utilities|IsValid (Variables|Default|GetConnectedActor)
    (:Is%20Not%20Valid
      (Actor|DestroyActor))))

(event Custom|SetGhostWheelSettingsServer
  (params (Settings :type Wheels%20Tool%20Actor%20Settings%20Structure))
  ;[1 1 1] GHOST WHEEL - Updating any parameters (run-time) - Technically a wheel only changes type at run-time but we keep it as example code
)

(event Custom|ShowDirectionIndicator
  (params (FwdDirection :type Boolean))
  ;[1 1 1] Spawn direction indicator
  (bind _returnvalue (Game|SpawnActorfromClass "/Game/CustomContent/UGC2281370083/Blueprints/Wheels/Props/WheelsDirectionPropBP.WheelsDirectionPropBP_C" (Transformation|GetActorTransform) "AlwaysSpawn" 0 FwdDirection 0))
  (bind _output_get (Variables|Default|SetWheelDirectionActor _returnvalue))
  (Transformation|AttachComponentToComponent _output_get (Variables|Default|GetConnectedComponent) "None" "KeepWorld" "KeepWorld" "KeepWorld" true))

(event Custom|ChangeDirectionMulticast
  ;[1 1 1] CHANGE DIRECTION MULTI-CAST - Actually changes the wheels velocity
  (Variables|Default|SetTorque (* (Variables|Default|GetTorque) -1.0))
  (CallFunction|ComputeTorqueVector))

(event Custom|SetWheelAttachment
  (params (Settings :type Wheels%20Tool%20Actor%20Settings%20Structure))
  (bind (_connectedactor _connectedcomponent _torque _forcelimit _friction _nocollision) (Utilities|Struct|BreakWheelsToolActorSettings Settings))
  ;[1 0.8798 0.3503] MULTICAST - Set up constraint
  (Variables|Default|SetConnectedActor _connectedactor)
  (Variables|Default|SetConnectedComponent _connectedcomponent)
  (Variables|Default|SetTorque _torque)
  (Variables|Default|SetForceLimit _forcelimit)
  (CallFunction|EnsureConnectionIsValid)
  (Collision|SetCollisionProfileName (Variables|Default|GetWheelMesh) "PhysicsActor" true :!class /Script/Engine.PrimitiveComponent)
  (Physics|SetSimulatePhysics (Variables|Default|GetWheelMesh) true)
  (Class|PhysicsConstraintComponent|SetConstrainedComponents (Variables|Default|GetPhysicsConstraint) (Variables|Default|GetWheelMesh) "None" (Variables|Default|GetConnectedComponent) "None")
  (Class|PhysicsConstraintComponent|SetDisableCollision (Variables|Default|GetPhysicsConstraint) _nocollision)
  (Utilities|HandleClientServerLogic
    (:ClientLogic
      (CallFunction|ShowDirectionIndicator true))))

(event EventTick
  (params (DeltaSeconds :type Float%20%28single-precision%29))
  (bind _connectedcomponent (Variables|Default|GetConnectedComponent))
  ;[1 1 1] EVENT TICK - Apply "torque"
  (Utilities|IsValid _connectedcomponent
    (:Is%20Valid
      (CallFunction|TouchGroundCheck DeltaSeconds)
      (if (Math|Boolean|ANDBoolean (Physics|IsSimulatingPhysics _connectedcomponent "None") (Variables|Default|GetGroundIsValid) (Variables|Default|GetbActive))
        (Class|PrimitiveComponent|AddForceatLocation (Variables|Default|GetConnectedComponent) (* (Math|Vector|RotateVectorAroundAxis (Math|Vector|GetForwardVector (Variables|Default|GetPhysicsConstraint)) 9e+01 (Math|Vector|GetUpVector (Variables|Default|GetConnectedComponent))) (* (Variables|Default|GetTorque) 1e+03)) (Transformation|GetWorldLocation (Variables|Default|GetWheelMesh)) "None")))))

(event EventActivated
  ;[1 1 1] Activation - TRIGGER INTERFACE
  (Variables|Default|SetbActive true))

(event EventDeactivated
  ;[1 1 1] Activation - TRIGGER INTERFACE
  (Variables|Default|SetbActive false))

(event EventBeginPlay
  ;[1 1 1] BEGIN PLAY - Should ghosted version..
)

(fn ConstructionScript)

(fn StoreBaseMaterialsandGhost
  (bind _wheelmesh (Variables|Default|GetWheelMesh))
  (bind _returnvalue (Rendering|Material|GetMaterials _wheelmesh))
  (Variables|BaseMaterials|SetBaseMaterials _returnvalue)
  (for (_ _array_index) _returnvalue
    (Rendering|Material|CreateDynamicMaterialInstance (Variables|Default|GetWheelMesh) _array_index "/Game/CustomContent/UGC2281370083/Blueprints/Wheels/Props/WheelOutlineMat.WheelOutlineMat" "None" :!class /Script/Engine.PrimitiveComponent)))

(fn ComputeTorqueVector
  (Variables|Default|SetComputedForce (Math|Vector|MakeVector (* (Variables|Default|GetTorque) 1e+03) 0.0 0.0)))

(fn TouchGroundCheck
  (params (Delta :type Float%20%28single-precision%29))
  (bind _wheelmesh (Variables|Default|GetWheelMesh))
  (bind _returnvalue (Transformation|GetWorldLocation _wheelmesh))
  ;[1 1 1] Check every X (50ms) for ground under use
  (bind _output_get (Variables|Default|SetGoundCheckTimeout (- (Variables|Default|GetGoundCheckTimeout) Delta)))
  (if (<= _output_get 0.0)
    (Variables|Default|SetGoundCheckTimeout (+ (Variables|Default|GetGoundCheckTimeout) 0.05))
    ;[1 1 1] Check ground is under wheel
    (bind _returnvalue_2 (Collision|LineTraceByChannel _returnvalue (- _returnvalue (Math|Vector|MakeVector 0.0 0.0 (Math|Vector|VectorLength (.Max (Components|StaticMesh|GetLocalBounds _wheelmesh))))) "TraceTypeQuery1" false (Utilities|Array|MakeArray (Variables|Default|GetConnectedActor)) "None"))
    (Variables|Default|SetGroundIsValid _returnvalue_2)))

(fn OnRepConnectedComponent
  (CallFunction|AttemptReplicatedAttach))

(fn AttemptReplicatedAttach
  ;[1 1 1] Not used
  (if (Math|Boolean|ANDBoolean (Utilities|IsValid (Variables|Default|GetPhysicsConstraint)) (Utilities|IsValid (Variables|Default|GetConnectedComponent)) (not (Ability|HasAuthority)))
    _))