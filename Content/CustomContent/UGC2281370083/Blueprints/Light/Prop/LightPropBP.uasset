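; Placeable light prop that previews as a ghost, then attaches to a target component as a physics-simulated point or spot light with a cable.
; Replicated Settings drive attachment through OnRep, spawning a physics constraint and, except on dedicated servers, applying cable, material and light visuals.
; Ghost setting edits are debounced on the owning client, then relayed via server to multicast.
; An authority timer destroys the prop when its connected actor becomes invalid.
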(event Custom|SetLightAttachedActor
  (params (Settings :type Light%20Tool%20Actor%20Settings%20Structure))
  ;[1 1 1] SERVER - Attach to actor (spawn physical constraint)
  (bind _output_get (Variables|Default|SetSettings Settings))
  (CallFunction|SetLightAttachment _output_get))

(event Custom|DebugSphere_
  (params (Center :type Vector))
  (Rendering|Debug|DrawDebugSphere Center 25.0 12 "(R=1.000000,G=0.104845,B=0.000000,A=1.000000)" 5.0 1.0))

(event Custom|SetGhostLightSettingsOwningClient
  (params (Settings :type Light%20Tool%20Actor%20Settings%20Structure))
  ;[1 1 1] GHOST LIGHT - cable length
  (Utilities|FlowControl|RetriggerableDelay 0.1) ; Stop flooding of network on lots of changes.. wait 100ms
  (CallFunction|SetGhostLightSettingsServer Settings))

(event Custom|EnsureConnectionIsValid
  ;[1 1 1] If conected to something, make sure it exists or delete ourselves
  (Networking|SwitchHasAuthority
    (:Authority
      (Utilities|Time|SetTimerbyEvent (delegate Custom|ConnectionCheck) 0.1 true))))

(event Custom|ConnectionCheck
  ;[1 1 1] If conected to something, make sure it exists or delete ourselves
  (Utilities|IsValid (Variables|Default|GetConnectedActor)
    (:Is%20Not%20Valid
      (Actor|DestroyActor))))

(event Custom|SetGhostLightSettingsServer
  (params (Settings :type Light%20Tool%20Actor%20Settings%20Structure))
  ;[1 1 1] GHOST LIGHT - cable length
  (CallFunction|SetGhostLightSettingsMulticast Settings))

(event Custom|SetGhostLightSettingsMulticast
  (params (Settings :type Light%20Tool%20Actor%20Settings%20Structure))
  (bind (_intensity _colour) (Utilities|Struct|BreakLightToolActorSettings Settings))
  (bind _cablelength (Utilities|Struct|BreakLightToolActorSettings Settings))
  (bind (_intensity_2 _colour_2 _spotlight _pointlight _attentuationradius _lockedconstraint _disableshadows) (Utilities|Struct|BreakLightToolActorSettings Settings))
  (bind _returnvalue (not _disableshadows))
  (bind _returnvalue_2 (/ _intensity 1.5e+03))
  ;[1 1 1] GHOST LIGHT - cable length
  (Utilities|FlowControl|Sequence
    (:then_0
      (Variables|/Script/CableComponent.CableComponent|SetEndLocation (Variables|Default|GetCable) (Math|Vector|MakeVector 0.0 0.0 _cablelength))
      (Rendering|SetVisibility (Variables|Default|GetCable) (> _cablelength 1e+01) false))
    (:then_1
      ;[1 1 1] Color setting
      (bind _returnvalue_3 (Rendering|Material|CreateDynamicMaterialInstance (Variables|Default|GetLitMesh) 0 "/Game/CustomContent/UGC2281370083/Blueprints/Light/Prop/Types/GlassLitMaterial.GlassLitMaterial" "None" :!class /Script/Engine.PrimitiveComponent)) ; light is always dynamic as we modify the param
      (Rendering|Material|SetVectorParameterValue _returnvalue_3 "ColorParam" _colour :!class /Script/Engine.MaterialInstanceDynamic)
      (Rendering|Material|SetScalarParameterValue _returnvalue_3 "Intensity" _returnvalue_2 :!class /Script/Engine.MaterialInstanceDynamic)
      (Rendering|SetVisibility (Variables|Default|GetLitMesh) (> _returnvalue_2 0.0) false))
    (:then_2
      ;[1 1 1] Set Light params (colour, dstance, intensity, etc.)
      (Utilities|FlowControl|Sequence
        (:then_0
          (Rendering|Components|Light|SetLightColor (Variables|Default|GetPointLight) _colour_2 true)
          (Rendering|Components|Light|SetIntensity (Variables|Default|GetPointLight) _intensity_2)
          (Rendering|SetVisibility (Variables|Default|GetPointLight) _pointlight false)
          (Rendering|Lighting|SetAttenuationRadius (Variables|Default|GetPointLight) _attentuationradius)
          (Rendering|Components|Light|SetCastShadows (Variables|Default|GetPointLight) _returnvalue))
        (:then_1
          (Rendering|Components|Light|SetLightColor (Variables|Default|GetSpotLight) _colour_2 true)
          (Rendering|Components|Light|SetIntensity (Variables|Default|GetSpotLight) _intensity_2)
          (Rendering|SetVisibility (Variables|Default|GetSpotLight) _spotlight false)
          (Rendering|Lighting|SetAttenuationRadius (Variables|Default|GetSpotLight) _attentuationradius)
          (Rendering|Components|Light|SetCastShadows (Variables|Default|GetSpotLight) _returnvalue))))))

(event Custom|SetLightAttachment
  (params (Settings :type Light%20Tool%20Actor%20Settings%20Structure))
  (bind (_connectedactor _connectedcomponent _cablelength _cableoffset _disablecollision) (Utilities|Struct|BreakLightToolActorSettings Settings))
  (bind _lightmesh (Variables|Default|GetLightMesh))
  (bind _cable (Variables|Default|GetCable))
  (bind (_intensity _colour) (Utilities|Struct|BreakLightToolActorSettings (Variables|Default|GetSettings)))
  (bind (_intensity_2 _colour_2 _spotlight _pointlight _attentuationradius) (Utilities|Struct|BreakLightToolActorSettings (Variables|Default|GetSettings)))
  (bind _lockedconstraint (Utilities|Struct|BreakLightToolActorSettings (Variables|Default|GetSettings)))
  (bind _returnvalue (/ _intensity 1.5e+03))
  (bind _returnvalue_2 (select _lockedconstraint "ACM_Locked" "ACM_Free"))
  ;[1 0.8798 0.3503] MULTICAST - Set up constraint
  (Variables|Default|SetConnectedActor _connectedactor)
  (Variables|Default|SetConnectedComponent _connectedcomponent)
  (Variables|Default|SetCableOffset _cableoffset)
  (Variables|Default|SetVerticalOffsetLocation _cablelength)
  (CallFunction|EnsureConnectionIsValid)
  (bind _returnvalue_3 (Game|SpawnActorfromClass "/Script/Engine.PhysicsConstraintActor" (Math|Transform|MakeTransform (+ (Transformation|GetActorLocation) (Math|Vector|MakeVector 0.0 0.0 (Variables|Default|GetVerticalOffsetLocation)))) "AlwaysSpawn" self 0))
  (Variables|Default|SetPhysicsConstrainsActor _returnvalue_3)
  (Physics|SetSimulatePhysics (Variables|Default|GetLightMesh) true)
  (if _disablecollision
    (Collision|SetCollisionProfileName _lightmesh "KJModNoCollisionSpawn" true :!class /Script/Engine.PrimitiveComponent)
    (else
      (Collision|SetCollisionProfileName _lightmesh "PhysicsActor" true :!class /Script/Engine.PrimitiveComponent)))
  (Networking|SwitchHasAuthority ; Server onlymake constraint
    (:Authority
      ;[1 1 1] Listen server?
      (if (Networking|IsDedicatedServer)
        ;[1 1 1] Create constraint and set it up
        (Utilities|IsValid (Variables|Default|GetConnectedComponent) :!label _label ; Valid? If not don't attach
          (:Is%20Valid
            (Class|PhysicsConstraintComponent|SetConstrainedComponents (Variables|/Script/Engine.PhysicsConstraintActor|GetConstraintComp (Variables|Default|GetPhysicsConstrainsActor)) (Variables|Default|GetLightMesh) "None" (Variables|Default|GetConnectedComponent) "None")
            (Class|PhysicsConstraintComponent|SetDisableCollision (Variables|/Script/Engine.PhysicsConstraintActor|GetConstraintComp (Variables|Default|GetPhysicsConstrainsActor)) true)
            (Class|PhysicsConstraintComponent|SetAngularTwistLimit (Variables|/Script/Engine.PhysicsConstraintActor|GetConstraintComp (Variables|Default|GetPhysicsConstrainsActor)) "ACM_Free" 0.0)
            (Class|PhysicsConstraintComponent|SetLinearXLimit (Variables|/Script/Engine.PhysicsConstraintActor|GetConstraintComp (Variables|Default|GetPhysicsConstrainsActor)) "LCM_Locked" 0.0)
            (Class|PhysicsConstraintComponent|SetLinearYLimit (Variables|/Script/Engine.PhysicsConstraintActor|GetConstraintComp (Variables|Default|GetPhysicsConstrainsActor)) "LCM_Locked" 0.0)
            (Class|PhysicsConstraintComponent|SetLinearZLimit (Variables|/Script/Engine.PhysicsConstraintActor|GetConstraintComp (Variables|Default|GetPhysicsConstrainsActor)) "LCM_Locked" 0.0)
            (Class|PhysicsConstraintComponent|SetAngularSwing1Limit (Variables|/Script/Engine.PhysicsConstraintActor|GetConstraintComp (Variables|Default|GetPhysicsConstrainsActor)) _returnvalue_2 0.0)
            (Class|PhysicsConstraintComponent|SetAngularSwing2Limit (Variables|/Script/Engine.PhysicsConstraintActor|GetConstraintComp (Variables|Default|GetPhysicsConstrainsActor)) _returnvalue_2 0.0)
            (Class|PhysicsConstraintComponent|SetAngularTwistLimit (Variables|/Script/Engine.PhysicsConstraintActor|GetConstraintComp (Variables|Default|GetPhysicsConstrainsActor)) _returnvalue_2 0.0)))
        (else
          (Utilities|FlowControl|Sequence :!label _label_2 ; Client does both
            (:then_0
              (goto _label))
            (:then_1
              ;[1 1 1] Client - Visualise light and cable
              (Utilities|IsValid (Variables|Default|GetConnectedComponent) ; Can be invalid and set attach crashes
                (:Is%20Valid
                  (Class|CableComponent|SetAttachEndtoComponent _cable (Variables|Default|GetConnectedComponent) "None")
                  (Variables|/Script/CableComponent.CableComponent|SetbAttachEnd _cable true)
                  (bind _output_get (Variables|/Script/CableComponent.CableComponent|SetCableLength (Variables|Default|GetCable) (/ (Variables|Default|GetVerticalOffsetLocation) 2.0)))
                  (Rendering|SetVisibility (Variables|Default|GetCable) (> _output_get 1e+01) false)
                  (Variables|/Script/CableComponent.CableComponent|SetEndLocation _cable (Variables|Default|GetCableOffset)))
                (:Is%20Not%20Valid
                  (Variables|/Script/CableComponent.CableComponent|SetbAttachEnd _cable true)))
              (Rendering|SetRenderCustomDepth (Variables|Default|GetLightMesh) false)
              (Rendering|SetRenderCustomDepth (Variables|Default|GetCable) false)
              (Rendering|Material|SetMaterial (Variables|Default|GetCable) 0 0)
              (Components|Activation|SetActive (Variables|Default|GetCable) true true)
              ;[1 1 1] Restore materials, set colour
              (bind _litmeshmaterial (CallFunction|RestoreBaseMaterials))
              (Rendering|Material|SetVectorParameterValue _litmeshmaterial "ColorParam" _colour :!class /Script/Engine.MaterialInstanceDynamic)
              (Rendering|Material|SetScalarParameterValue _litmeshmaterial "Intensity" _returnvalue :!class /Script/Engine.MaterialInstanceDynamic)
              (Rendering|SetVisibility (Variables|Default|GetLitMesh) (> _returnvalue 0.0) false)
              ;[1 1 1] Set Light params (colour, dstance, intensity, etc.)
              (Utilities|FlowControl|Sequence
                (:then_0
                  (Rendering|Components|Light|SetLightColor (Variables|Default|GetPointLight) _colour_2 true)
                  (Rendering|Components|Light|SetIntensity (Variables|Default|GetPointLight) _intensity_2)
                  (Rendering|SetVisibility (Variables|Default|GetPointLight) _pointlight false)
                  (Rendering|Lighting|SetAttenuationRadius (Variables|Default|GetPointLight) _attentuationradius))
                (:then_1
                  (Rendering|Components|Light|SetLightColor (Variables|Default|GetSpotLight) _colour_2 true)
                  (Rendering|Components|Light|SetIntensity (Variables|Default|GetSpotLight) _intensity_2)
                  (Rendering|SetVisibility (Variables|Default|GetSpotLight) _spotlight false)
                  (Rendering|Lighting|SetAttenuationRadius (Variables|Default|GetSpotLight) _attentuationradius))))))))
    (:Remote
      (goto _label_2))))

(event EventBeginPlay
  ;[1 1 1] BEGIN PLAY - Should ghosted version..
  (if (not (!= (.ConnectedActor (Utilities|Struct|BreakLightToolActorSettings (Variables|Default|GetSettings))) 0)) ; Have we been spawned knowing our target?
    (CallFunction|StoreBaseMaterialsandGhost) ; No store materials, and go ghost
    (Rendering|Components|Light|SetIntensity (Variables|Default|GetPointLight) 0.0)))

(fn ConstructionScript)

(fn OnRepSettings
  (CallFunction|SetLightAttachment (Variables|Default|GetSettings)))

(fn StoreBaseMaterialsandGhost
  (bind _lightmesh (Variables|Default|GetLightMesh))
  (bind _returnvalue (Rendering|Material|GetMaterials _lightmesh))
  (Variables|Default|SetMaterialsModified true)
  (Variables|BaseMaterials|SetBaseMaterials _returnvalue)
  (for (_ _array_index) _returnvalue
    (Rendering|Material|CreateDynamicMaterialInstance (Variables|Default|GetLightMesh) _array_index 0 "None" :!class /Script/Engine.PrimitiveComponent))
  (Variables|BaseMaterials|SetLitMeshMaterial (Rendering|Material|GetMaterial (Variables|Default|GetLitMesh) 0))
  (Rendering|Material|CreateDynamicMaterialInstance (Variables|Default|GetLitMesh) 0 0 "None" :!class /Script/Engine.PrimitiveComponent)
  (Rendering|Material|CreateDynamicMaterialInstance (Variables|Default|GetCable) 0 0 "None" :!class /Script/Engine.PrimitiveComponent))

(fn RestoreBaseMaterials
  (bind _basematerials (Variables|BaseMaterials|GetBaseMaterials))
  (if (Variables|Default|GetMaterialsModified) ; Have we been a ghost? if so restore all materials
    (for (_ _array_index) _basematerials
      (Rendering|Material|CreateDynamicMaterialInstance (Variables|Default|GetLightMesh) _array_index (Utilities|Array|Get(acopy) _basematerials) "None" :!class /Script/Engine.PrimitiveComponent))
    (Rendering|Material|CreateDynamicMaterialInstance (Variables|Default|GetCable) 0 0 "None" :!class /Script/Engine.PrimitiveComponent))
  (bind _returnvalue (Rendering|Material|CreateDynamicMaterialInstance (Variables|Default|GetLitMesh) 0 "/Game/CustomContent/UGC2281370083/Blueprints/Light/Prop/Types/GlassLitMaterial.GlassLitMaterial" "None" :!class /Script/Engine.PrimitiveComponent)) ; light is always dynamic as we modify the param
  (return _returnvalue))