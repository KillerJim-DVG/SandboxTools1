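; Player tool that places configurable lights, either static or tied by a cord to a prop.
; Each tick the local client traces from the camera, positions a ghost preview light and sends the target and scaled local cable offset to the server.
; Left click spawns the real light, which the server attaches, and replication records it in removal history.
; Saved and widget-edited settings sync to server and ghost; type changes respawn the ghost.
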(event Custom|AdjustGhostLightSettings
  (params (Settings :type Light%20Tool%20Actor%20Settings%20Structure))
  ;[1 1 1] GHOST LIGHT - changes
  (Utilities|IsValid (Variables|Ghosting|GetGhostLight)
    (:Is%20Valid
      (Default|SetGhostLightSettingsOwningClient (Variables|Ghosting|GetGhostLight) Settings))))

(event Custom|UpdateHistoryOwningClient
  (params (ObjectToAttach :type Actor%20Object%20Reference))
  ;[1 1 1] Update the history (to reflect last selection as most recent)
  (Class|KJModToolProxy|AddHistoryEntry (Utilities|Struct|MakeKJModToolHistoryItem ObjectToAttach "Removing light " "Light" "DeleteItem")))

(event Custom|SetLightInformationOwningClient
  (params (Location :type Vector) (Visible :type Boolean) (TargetActor :type Actor%20Object%20Reference) (TargetComponent :type Primitive%20Component%20Object%20Reference) (CableOffset :type Vector) (Rotation :type Rotator))
  (bind _ghostlight (Variables|Ghosting|GetGhostLight))
  ;[1 1 1] Update light position and settings information (local and remote)
  (CallFunction|SetLightInformationServer Location Visible TargetActor TargetComponent CableOffset Rotation)
  (Utilities|IsValid _ghostlight ; may not be replicated yet
    (:Is%20Valid
      (Transformation|SetActorLocation _ghostlight Location false true)
      (Transformation|SetActorRotation _ghostlight Rotation true)
      (Rendering|SetActorHiddenInGame _ghostlight (not Visible)))))

(event Custom|SetLightInformationServer
  (params (Location :type Vector) (Visible :type Boolean) (TargetActor :type Actor%20Object%20Reference) (TargetComponent :type Primitive%20Component%20Object%20Reference) (CableOffset :type Vector) (Rotation :type Rotator))
  (bind _ghostlight (Variables|Ghosting|GetGhostLight))
  ;[1 1 1] Update light position and settings information (local and remote)
  (Utilities|Struct|SetmembersinLightToolActorSettings (Variables|ToolSetting|GetSettings) TargetActor TargetComponent CableOffset)
  (Utilities|IsValid _ghostlight ; Is null when switching lamp's
    (:Is%20Valid
      (Transformation|SetActorLocation _ghostlight Location false true)
      (Transformation|SetActorRotation _ghostlight Rotation true)
      (Rendering|SetActorHiddenInGame _ghostlight (not Visible)))))

(event EventDestroyed
  (bind _ghostlight (Variables|Ghosting|GetGhostLight))
  ;[1 1 1] DESTROYED - remove ghost light from server
  (Utilities|IsValid _ghostlight
    (:Is%20Valid
      (Actor|DestroyActor _ghostlight))))

(event EventBeginPlay
  ;[0.9593 1 0.1335] BEGIN PLAY EVENT
  (Networking|SwitchHasAuthority
    (:Authority
      ;;[1 1 1] Listen server?
      (if (not (Networking|IsDedicatedServer))
        (Utilities|FlowControl|Sequence
          (:then_1
            ;;[1 1 1] If local controlled; init once..
            (Utilities|IsLocallyControlled :!label _label
              (:LocalControl
                (CallFunction|NotifyOwnerOfInstantiation)
                (if (not (Variables|Initialisation|GetInitialised))
                  (Variables|Initialisation|SetInitialised true)
                  ;;[1 1 1] Reload settings
                  (CallFunction|CreateandShowToolsAssistInformation)
                  (CallFunction|InitSettings)
                  ;;[1 1 1] Create ghost light
                  (CallFunction|CreateGhostLight (.Type (Utilities|Struct|BreakLightToolActorSettings (Variables|ToolSetting|GetSettings)))))))))))
    (:Remote
      (goto _label))))

(event EventTick
  (params (DeltaSeconds :type Float%20%28single-precision%29))
  (bind _settings (Variables|ToolSetting|GetSettings))
  (bind (_cablelength _attentuationradius _lockedconstraint) (Utilities|Struct|BreakLightToolActorSettings _settings))
  ;[1 1 1] EVENT TICK
  (|CallParentFunction DeltaSeconds)
  (Utilities|IsLocallyControlled
    (:LocalControl
      (Utilities|HandleClientServerLogic
        (:ClientLogic
          ;;[1 1 1] Handle MOUSE SELECTION POINT
          (bind _returnvalue (Class|KJModToolProxy|GetPawnCameraComponent))
          (bind (_outhit _returnvalue_2) (Collision|LineTraceByChannel (Transformation|GetWorldLocation _returnvalue) (+ (Transformation|GetWorldLocation _returnvalue) (* (Math|Vector|GetForwardVector _returnvalue) 3.5e+03)) "TraceTypeQuery1" true (Utilities|Array|MakeArray (Game|Player|GetPlayerPawn 0)) "None"))
          (if _returnvalue_2
            (Utilities|IsValid (.HitActor (Collision|BreakHitResult _outhit))
              (:Is%20Valid
                (Utilities|IsValid (Variables|Ghosting|GetGhostLight) ; May not be replicated from server (yet)
                  (:Is%20Valid
                    (bind _rotation (Utilities|BuildRotationfromImpactNormal (.ImpactPoint (Collision|BreakHitResult _outhit)) (.ImpactNormal (Collision|BreakHitResult _outhit)))
                      (:Out
                        (Variables|Ghosting|SetGhostLightLocation (- (.Location (Collision|BreakHitResult _outhit)) (Math|Vector|MakeVector 0.0 0.0 _cablelength)))
                        (Variables|Ghosting|SetGhostLightRotation (select _lockedconstraint _rotation "0, 0, 0"))
                        (bind _output_get (Variables|Ghosting|SetCableLocalLocation (/ (Math|Vector|UnrotateVector (- (.ImpactPoint (Collision|BreakHitResult _outhit)) (Transformation|GetWorldLocation (.HitComponent (Collision|BreakHitResult _outhit)))) (Transformation|GetWorldRotation (.HitComponent (Collision|BreakHitResult _outhit)))) (Transformation|GetWorldScale (.HitComponent (Collision|BreakHitResult _outhit))))))
                        (CallFunction|SetLightInformationOwningClient (Variables|Ghosting|GetGhostLightLocation) true (.HitActor (Collision|BreakHitResult _outhit)) (.HitComponent (Collision|BreakHitResult _outhit)) _output_get (Variables|Ghosting|GetGhostLightRotation))
                        (Variables|Ghosting|SetGhostLightVisible true))))
                  (:Is%20Not%20Valid
                    (CallFunction|SetLightInformationOwningClient "0, 0, 0" false 0 0 "0, 0, 0" "0, 0, 0" :!label _label)
                    (Variables|Ghosting|SetGhostLightVisible false))))
              (:Is%20Not%20Valid
                (goto _label)))
            (else
              (goto _label))))))))

(event Custom|NotifyServerOfGhostLight
  (params (GhostLight :type Light%20Prop%20BP%20Object%20Reference))
  ;[1 1 1] Server - Record ghost light for removal
  (Variables|Ghosting|SetGhostLight GhostLight))

(event Custom|ServerReleaseLight
  (params (LightToRelease :type Light%20Prop%20BP%20Object%20Reference))
  ;[1 1 1] SERVER - Release Light
  (Default|SetLightAttachedActor LightToRelease (Variables|ToolSetting|GetSettings)))

(event EventToolProxyItemSpawned
  (params (spawnedActor :type Actor%20Object%20Reference))
  (bind _settings (Variables|ToolSetting|GetSettings))
  (bind (_cablelength _type) (Utilities|Struct|BreakLightToolActorSettings _settings))
  ;[1 1 1] (interface) Item Spawned - From Pawn
  (bind _aslight_prop_bp (Utilities|Casting|CastToLightPropBP spawnedActor)
    (:then
      (Utilities|IsValid (Variables|Ghosting|GetGhostLight) ; First time? it's our "ghost" light
        (:Is%20Valid
          (bind _output_get (Variables|Spawning|SetSpawnedActor_0 _aslight_prop_bp))
          (CallFunction|ServerReleaseLight _output_get) ; A real light has been spawned
        )
        (:Is%20Not%20Valid
          (Variables|Ghosting|SetGhostLight _aslight_prop_bp)
          (CallFunction|SettingSetType _type) ; When 1st spawning something (the ghost) set it's initial mesh
          (CallFunction|SettingSetCableLength _cablelength))))
    (:CastFailed
      (|CallParentFunction spawnedActor) ; Probably a Q menu spawning; let parent deal with it
    )))

(event EventToolProxyPrimaryMouseClick
  (params (pressed :type Boolean))
  ;[1 1 1] LEFT/RIGHT MOUSE - Drop or freeze if anything on tool
  ;;[1 1 1] Left - Attempt Grab or Release any object
  (if pressed ; Pressed?
    (Utilities|IsValid (Variables|Ghosting|GetGhostLight)
      (:Is%20Valid
        (if (Variables|Ghosting|GetGhostLightVisible)
          (if (<= (Variables|Default|GetRespawnDelayTimeout) 0.0)
            (Class|KJModToolProxy|SpawnItem (Utilities|Struct|BreakLightToolActorSettings (Variables|ToolSetting|GetSettings)) (Variables|Ghosting|GetGhostLightLocation) (Variables|Ghosting|GetGhostLightRotation) "1.000000,1.000000,1.000000")
            (Variables|Default|SetRespawnDelayTimeout 0.5)))))
    (elif (Variables|/Script/Engine.PlayerController|GetbShowMouseCursor (Game|GetPlayerController 0)) ; If on Q window, or anything else, do not drop
      _)))

(event Custom|Setting_SetCableLength
  (params (Value :type Float%20%28single-precision%29))
  ;[1 1 1] Settings (from widgets and onload)
  (bind _structout (Utilities|Struct|SetmembersinLightToolActorSettings (Variables|ToolSetting|GetSettings) Value))
  (CallFunction|AdjustGhostLightSettings _structout)
  ;[1 1 1] Update server
  (if (Variables|ToolSetting|GetbServerSettingsInited)
    (CallFunction|SetLightSettingsOwningClient (Variables|ToolSetting|GetSettings))))

(event Custom|Setting_SetColor
  (params (Color :type Linear%20Color%20Structure))
  ;[1 1 1] Settings (from widgets and onload)
  (bind _structout (Utilities|Struct|SetmembersinLightToolActorSettings (Variables|ToolSetting|GetSettings) Color))
  (CallFunction|AdjustGhostLightSettings _structout)
  ;[1 1 1] Update server
  (if (Variables|ToolSetting|GetbServerSettingsInited)
    (CallFunction|SetLightSettingsOwningClient (Variables|ToolSetting|GetSettings))))

(event Custom|SetLightActorBP
  (params (Type :type String))
  (CallFunction|RemovePreviousLightActorBP (Variables|Ghosting|GetGhostLight) Type))

(event Custom|Setting_EnableSpotLight
  (params (Enabled :type Boolean))
  ;[1 1 1] Settings (from widgets and onload)
  (bind _structout (Utilities|Struct|SetmembersinLightToolActorSettings (Variables|ToolSetting|GetSettings) Enabled))
  (CallFunction|AdjustGhostLightSettings _structout)
  ;[1 1 1] Update server
  (if (Variables|ToolSetting|GetbServerSettingsInited)
    (CallFunction|SetLightSettingsOwningClient (Variables|ToolSetting|GetSettings))))

(event Custom|Setting_LockedConstraint
  (params (Locked :type Boolean))
  ;[1 1 1] Settings (from widgets and onload)
  (Utilities|Struct|SetmembersinLightToolActorSettings (Variables|ToolSetting|GetSettings) Locked)
  ;[1 1 1] Update server
  (if (Variables|ToolSetting|GetbServerSettingsInited)
    (CallFunction|SetLightSettingsOwningClient (Variables|ToolSetting|GetSettings))))

(event Custom|Setting_EnablePointLight
  (params (Enabled :type Boolean))
  ;[1 1 1] Settings (from widgets and onload)
  (bind _structout (Utilities|Struct|SetmembersinLightToolActorSettings (Variables|ToolSetting|GetSettings) Enabled))
  (CallFunction|AdjustGhostLightSettings _structout)
  ;[1 1 1] Update server
  (if (Variables|ToolSetting|GetbServerSettingsInited)
    (CallFunction|SetLightSettingsOwningClient (Variables|ToolSetting|GetSettings))))

(event Custom|Setting_AttenuationRadius
  (params (Radius :type Float%20%28single-precision%29))
  ;[1 1 1] Settings (from widgets and onload)
  (bind _structout (Utilities|Struct|SetmembersinLightToolActorSettings (Variables|ToolSetting|GetSettings) Radius))
  (CallFunction|AdjustGhostLightSettings _structout)
  ;[1 1 1] Update server
  (if (Variables|ToolSetting|GetbServerSettingsInited)
    (CallFunction|SetLightSettingsOwningClient (Variables|ToolSetting|GetSettings))))

(event Custom|Setting_SetIntensity
  (params (Value :type Float%20%28single-precision%29))
  ;[1 1 1] Settings (from widgets and onload)
  (bind _structout (Utilities|Struct|SetmembersinLightToolActorSettings (Variables|ToolSetting|GetSettings) Value))
  (CallFunction|AdjustGhostLightSettings _structout)
  ;[1 1 1] Update server
  (if (Variables|ToolSetting|GetbServerSettingsInited)
    (CallFunction|SetLightSettingsOwningClient (Variables|ToolSetting|GetSettings))))

(event Custom|RemovePreviousLightActorBP
  (params (Actor :type Actor%20Object%20Reference) (Type :type String))
  (Utilities|IsValid Actor
    (:Is%20Valid
      (Actor|DestroyActor Actor)
      (Variables|Ghosting|SetGhostLight 0)
      (Utilities|FlowControl|Delay 0.25)
      (CallFunction|ReInitLightActor Type))))

(event Custom|Setting_DisableCollision
  (params (DisableCollision :type Boolean))
  ;[1 1 1] Settings (from widgets and onload)
  (Utilities|Struct|SetmembersinLightToolActorSettings (Variables|ToolSetting|GetSettings) DisableCollision)
  ;[1 1 1] Update server
  (if (Variables|ToolSetting|GetbServerSettingsInited)
    (CallFunction|SetLightSettingsOwningClient (Variables|ToolSetting|GetSettings))))

(event Custom|SetLightSettingsOwningClient
  (params (Settings :type Light%20Tool%20Actor%20Settings%20Structure))
  ;[1 1 1] Replicate changes (and visualise mesh)
  (CallFunction|SetLightSettingsServer Settings))

(event Custom|Setting_SetType
  (params (Type :type String))
  ;[1 1 1] Settings (from widgets and onload)
  (if (Utilities|Enum|NotEqual(Enum) Type (.Type (Utilities|Struct|BreakLightToolActorSettings (Variables|ToolSetting|GetSettings)))) ; Did they change the visualisation?
    (CallFunction|SetLightActorBP Type))
  (Utilities|Struct|SetmembersinLightToolActorSettings (Variables|ToolSetting|GetSettings) Type)
  ;[1 1 1] Update server
  (if (Variables|ToolSetting|GetbServerSettingsInited)
    (CallFunction|SetLightSettingsOwningClient (Variables|ToolSetting|GetSettings))))

(event Custom|SetLightSettingsServer
  (params (Settings :type Light%20Tool%20Actor%20Settings%20Structure))
  ;[1 1 1] Replicate changes (and visualise mesh)
  (Variables|ToolSetting|SetSettings Settings))

(event Custom|ReInitLightActor
  (params (Type :type String))
  (CallFunction|CreateGhostLight Type))

(event Custom|Setting_DisableShadows
  (params (DisableShadows :type Boolean))
  ;[1 1 1] Settings (from widgets and onload)
  (bind _structout (Utilities|Struct|SetmembersinLightToolActorSettings (Variables|ToolSetting|GetSettings) DisableShadows))
  (CallFunction|AdjustGhostLightSettings _structout)
  ;[1 1 1] Update server
  (if (Variables|ToolSetting|GetbServerSettingsInited)
    (CallFunction|SetLightSettingsOwningClient (Variables|ToolSetting|GetSettings))))

(event Custom|InitSettings
  ;[1 1 1] Init / Load previous settings
  (bind _returnvalue (Class|KJModToolProxy|LoadToolSettings "LightToolSettings"))
  (Utilities|IsValid _returnvalue ; No save? use defaults
    (:Is%20Valid
      (bind _aslight_tool_save_game_bp (Utilities|Casting|CastToLightToolSaveGameBP _returnvalue)
        (:then
          (Utilities|FlowControl|Sequence
            (:then_0
              ;[1 1 1] Local Initial settings
              (Utilities|FlowControl|Sequence
                (:then_0
                  (CallFunction|SettingSetIntensity (Variables|/Game/CustomContent/UGC2281370083/Blueprints/Light/LightToolSaveGameBP.LightToolSaveGameBP_C|GetIntensity _aslight_tool_save_game_bp)))
                (:then_1
                  (CallFunction|SettingSetColor (Variables|/Game/CustomContent/UGC2281370083/Blueprints/Light/LightToolSaveGameBP.LightToolSaveGameBP_C|GetColor _aslight_tool_save_game_bp)))
                (:then_2
                  (CallFunction|SettingSetCableLength (Variables|/Game/CustomContent/UGC2281370083/Blueprints/Light/LightToolSaveGameBP.LightToolSaveGameBP_C|GetCableLength _aslight_tool_save_game_bp)))
                (:then_3
                  (CallFunction|SettingSetType (Variables|/Game/CustomContent/UGC2281370083/Blueprints/Light/LightToolSaveGameBP.LightToolSaveGameBP_C|GetType _aslight_tool_save_game_bp)))
                (:then_4
                  (CallFunction|SettingDisableCollision (Variables|/Game/CustomContent/UGC2281370083/Blueprints/Light/LightToolSaveGameBP.LightToolSaveGameBP_C|GetbDisableCollision _aslight_tool_save_game_bp)))
                (:then_5
                  (CallFunction|SettingEnableSpotLight (Variables|/Game/CustomContent/UGC2281370083/Blueprints/Light/LightToolSaveGameBP.LightToolSaveGameBP_C|GetbSpotLight _aslight_tool_save_game_bp)))
                (:then_6
                  (CallFunction|SettingEnablePointLight (Variables|/Game/CustomContent/UGC2281370083/Blueprints/Light/LightToolSaveGameBP.LightToolSaveGameBP_C|GetbPointLight _aslight_tool_save_game_bp)))
                (:then_7
                  (CallFunction|SettingLockedConstraint (Variables|/Game/CustomContent/UGC2281370083/Blueprints/Light/LightToolSaveGameBP.LightToolSaveGameBP_C|GetbLockedConstraint _aslight_tool_save_game_bp)))
                (:then_8
                  (CallFunction|SettingAttenuationRadius (Variables|/Game/CustomContent/UGC2281370083/Blueprints/Light/LightToolSaveGameBP.LightToolSaveGameBP_C|GetAttenutationRadius _aslight_tool_save_game_bp)))
                (:then_9
                  (CallFunction|SettingDisableShadows (Variables|/Game/CustomContent/UGC2281370083/Blueprints/Light/LightToolSaveGameBP.LightToolSaveGameBP_C|GetbDisableShadow _aslight_tool_save_game_bp)))))
            (:then_1
              ;[1 1 1] Init settings server
              (CallFunction|SetLightSettingsOwningClient (Variables|ToolSetting|GetSettings) :!label _label)
              (Variables|ToolSetting|SetbServerSettingsInited true))))
        (:CastFailed
          (goto _label))))
    (:Is%20Not%20Valid
      (goto _label))))

(fn ConstructionScript)

(fn CreateandShowToolsAssistInformation
  (Class|KJModToolProxy|ShowToolAssistUI)
  (Class|KJModToolProxy|SetToolAssistTitle "Light" "A light that can be static or tied, via a cord, to any prop")
  (Class|KJModToolProxy|ClearToolAssistFunctions)
  (bind _returnvalue (Class|KJModToolProxy|CreateToolAssistFunction "Add light at required point"))
  (Class|KJModToolProxy|SetToolAssistFunctionPrimaryDetails _returnvalue "LeftMouse"))

(fn CreateGhostLight
  (params (AssetPath :type String))
  (bind _returnvalue (Game|GetPlayerCameraManager 0))
  (Class|KJModToolProxy|SpawnItem AssetPath (+ (Transformation|GetActorLocation _returnvalue) (* (Transformation|GetActorForwardVector _returnvalue) 5e+02)) "0, 0, 0" "1.000000,1.000000,1.000000"))

(fn OnRepSpawnedActor0
  (bind _spawnedactor_0 (Variables|Spawning|GetSpawnedActor_0))
  ;[1 1 1] If we're the owner then record the lights creation in our history (for delete)
  (Utilities|IsLocallyControlled
    (:LocalControl
      (Utilities|IsValid _spawnedactor_0
        (:Is%20Valid
          (CallFunction|UpdateHistoryOwningClient _spawnedactor_0))))))

(fn ToolProxyGetToolSettingPanel
  (Utilities|IsValid (Variables|ToolSetting|GetToolSettingsWidget)
    (:Is%20Valid
      _)
    (:Is%20Not%20Valid
      (bind _returnvalue (UserInterface|CreateWidget "/Game/CustomContent/UGC2281370083/Blueprints/Light/Settings/LightToolSettingsWidgetBP.LightToolSettingsWidgetBP_C" (Game|GetPlayerController 0) self))
      (Default|CreatedEvent _returnvalue)
      (Variables|ToolSetting|SetToolSettingsWidget _returnvalue)))
  (return (Variables|ToolSetting|GetToolSettingsWidget)))