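; Player tool that places configurable 3D text props on surfaces in the world.
; The local client traces from the camera each tick, moving a ghost TextPropBP aligned to the hit normal and mirroring it to the server.
; Left click spawns the text with a short cooldown; the server applies current settings and OnRep records it in undo history.
; Settings load from a save game or change through the widget, updating ghost and server.
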(event Custom|AdjustGhostTextSettings
  (params (Settings :type Text%20Tool%20Actor%20Settings%20Structure))
  ;[1 1 1] GHOST TEXT - changes
  (Utilities|IsValid (Variables|Ghosting|GetGhostText)
    (:Is%20Valid
      (Default|SetGhostTextSettingsOwningClient (Variables|Ghosting|GetGhostText) Settings))))

(event Custom|UpdateHistoryOwningClient
  (params (ObjectToAttach :type Actor%20Object%20Reference))
  ;[1 1 1] Update the history (to reflect last selection as most recent)
  (Class|KJModToolProxy|AddHistoryEntry (Utilities|Struct|MakeKJModToolHistoryItem ObjectToAttach "Removing text " "Text" "DeleteItem")))

(event Custom|SetGhostTextInformationOwningClient
  (params (IsVisible :type Boolean) (Location :type Vector) (Rotation :type Rotator))
  (bind _ghosttext (Variables|Ghosting|GetGhostText))
  ;[1 1 1] Ghost Text Update - Update text position and settings information (local and remote)
  (CallFunction|SetGhostTextInformationServer IsVisible Location Rotation)
  (Utilities|IsValid _ghosttext ; may not be replicated yet
    (:Is%20Valid
      (Transformation|SetActorLocation _ghosttext Location false true)
      (Transformation|SetActorRotation _ghosttext Rotation true)
      (Rendering|SetActorHiddenInGame _ghosttext (not IsVisible)))))

(event Custom|SetGhostTextInformationServer
  (params (Visible :type Boolean) (Location :type Vector) (Rotation :type Rotator))
  (bind _ghosttext (Variables|Ghosting|GetGhostText))
  ;[1 1 1] Ghost Text Update - Update text position and settings information (local and remote)
  (Utilities|IsValid _ghosttext ; Is null when switching lamp's
    (:Is%20Valid
      (Transformation|SetActorLocation _ghosttext Location false true)
      (Transformation|SetActorRotation _ghosttext Rotation true)
      (Rendering|SetActorHiddenInGame _ghosttext (not Visible)))))

(event EventDestroyed
  (bind _ghosttext (Variables|Ghosting|GetGhostText))
  ;[1 1 1] DESTROYED - remove ghost text from server
  (Utilities|IsValid _ghosttext
    (:Is%20Valid
      (Actor|DestroyActor _ghosttext))))

(event EventBeginPlay
  ;[0.9593 1 0.1335] BEGIN PLAY EVENT
  (Utilities|HandleClientServerLogic
    (:ClientLogic
      ;;[1 1 1] If local controlled; init once..
      (Utilities|IsLocallyControlled
        (:LocalControl
          (CallFunction|NotifyOwnerOfInstantiation)
          (if (not (Variables|Initialisation|GetInitialised))
            (Variables|Initialisation|SetInitialised true)
            ;;[1 1 1] Reload settings
            (CallFunction|CreateandShowToolsAssistInformation)
            (CallFunction|InitSettings)
            ;;[1 1 1] Create ghost text
            (CallFunction|CreateGhostText)))))))

(event EventTick
  (params (DeltaSeconds :type Float%20%28single-precision%29))
  ;[1 1 1] EVENT TICK
  (|CallParentFunction DeltaSeconds)
  (Utilities|IsLocallyControlled
    (:LocalControl
      (Utilities|HandleClientServerLogic
        (:ClientLogic
          ;;[1 1 1] Handle MOUSE SELECTION POINT
          (bind _returnvalue (Class|KJModToolProxy|GetPawnCameraComponent))
          (bind (_outhit _returnvalue_2) (Collision|LineTraceByChannel (Transformation|GetWorldLocation _returnvalue) (+ (Transformation|GetWorldLocation _returnvalue) (* (Math|Vector|GetForwardVector _returnvalue) 3.5e+03)) "TraceTypeQuery1" true (Utilities|Array|MakeArray (Game|Player|GetPlayerPawn 0) (Variables|Ghosting|GetGhostText)) "None"))
          (if _returnvalue_2
            (Utilities|IsValid (.HitActor (Collision|BreakHitResult _outhit))
              (:Is%20Valid
                (Utilities|IsValid (Variables|Ghosting|GetGhostText) ; May not be replicated from server (yet)
                  (:Is%20Valid
                    (bind _structout (Utilities|Struct|SetmembersinTextToolActorSettings (Variables|ToolSetting|GetRunTimeSettings) (.HitActor (Collision|BreakHitResult _outhit)))) ; Record "hit" actor so any attach functionality (when real Text is created on click) has it..
                    (Variables|ToolSetting|SetRunTimeSettings _structout)
                    (bind _rotation (Utilities|BuildRotationfromImpactNormal (.ImpactPoint (Collision|BreakHitResult _outhit)) (.ImpactNormal (Collision|BreakHitResult _outhit)))
                      (:Out
                        (Variables|Ghosting|SetGhostTextLocation (- (.Location (Collision|BreakHitResult _outhit)) (* (Math|Vector|GetForwardVector _rotation) (.ZOffset (Utilities|Struct|BreakTextToolActorSettings (Variables|ToolSetting|GetRunTimeSettings))))))
                        (Variables|Ghosting|SetGhostTextRotation _rotation)
                        (Variables|Ghosting|SetCableLocalLocation (/ (Math|Vector|UnrotateVector (- (.ImpactPoint (Collision|BreakHitResult _outhit)) (Transformation|GetWorldLocation (.HitComponent (Collision|BreakHitResult _outhit)))) (Transformation|GetWorldRotation (.HitComponent (Collision|BreakHitResult _outhit)))) (Transformation|GetWorldScale (.HitComponent (Collision|BreakHitResult _outhit)))))
                        (CallFunction|SetGhostTextInformationOwningClient true (Variables|Ghosting|GetGhostTextLocation) (Variables|Ghosting|GetGhostTextRotation))
                        (Variables|Ghosting|SetGhostTextVisible true))))
                  (:Is%20Not%20Valid
                    (CallFunction|SetGhostTextInformationOwningClient false "0, 0, 0" "0, 0, 0" :!label _label)
                    (Variables|Ghosting|SetGhostTextVisible false))))
              (:Is%20Not%20Valid
                (goto _label)))
            (else
              (goto _label))))))))

(event Custom|ServerReleaseText
  (params (TextToRelease :type Text%20Prop%20BP%20Object%20Reference))
  ;[1 1 1] SERVER - Release Text; we need to set it's settings so they are set (and it visualises itself correctly)
  (Variables|/Game/CustomContent/UGC2281370083/Blueprints/TextTool/Prop/TextPropBP.TextPropBP_C|SetSettings TextToRelease (Variables|ToolSetting|GetRunTimeSettings)))

(event EventToolProxyItemSpawned
  (params (spawnedActor :type Actor%20Object%20Reference))
  ;[1 1 1] (interface) Item Spawned - From Pawn
  (bind _astext_prop_bp (Utilities|Casting|CastToTextPropBP spawnedActor)
    (:then
      (Utilities|IsValid (Variables|Ghosting|GetGhostText) ; First time? it's our "ghost" text
        (:Is%20Valid
          (bind _output_get (Variables|Spawning|SetSpawnedTextActor _astext_prop_bp))
          (CallFunction|ServerReleaseText _output_get))
        (:Is%20Not%20Valid
          (Variables|Ghosting|SetGhostText _astext_prop_bp)
          (CallFunction|AdjustGhostTextSettings (Variables|ToolSetting|GetRunTimeSettings)))))
    (:CastFailed
      (|CallParentFunction spawnedActor) ; Probably a Q menu spawning; let parent deal with it
    )))

(event EventToolProxyPrimaryMouseClick
  (params (pressed :type Boolean))
  ;[1 1 1] LEFT/RIGHT MOUSE - Drop or freeze if anything on tool
  ;;[1 1 1] Left - Attempt Grab or Release any object
  (if pressed ; Pressed?
    (Utilities|IsValid (Variables|Ghosting|GetGhostText)
      (:Is%20Valid
        (if (Variables|Ghosting|GetGhostTextVisible)
          (if (<= (Variables|Default|GetRespawnDelayTimeout) 0.0)
            (Class|KJModToolProxy|SpawnItem "/Game/CustomContent/UGC2281370083/Blueprints/TextTool/Prop/TextPropBP" (Variables|Ghosting|GetGhostTextLocation) (Variables|Ghosting|GetGhostTextRotation) "1.000000,1.000000,1.000000")
            (Class|KJModToolProxy|PlayToolSoundEffect "ToolSpawnSound" true)
            (Variables|Default|SetRespawnDelayTimeout 0.5)))))
    (elif (Variables|/Script/Engine.PlayerController|GetbShowMouseCursor (Game|GetPlayerController 0)) ; If on Q window, or anything else, do not drop
      _)))

(event Custom|Setting_SetZOffset
  (params (ZOffset :type Float%20%28single-precision%29))
  ;[1 1 1] Settings (from widgets and onload)
  (bind _structout (Utilities|Struct|SetmembersinTextToolActorSettings (Variables|ToolSetting|GetRunTimeSettings) ZOffset))
  (CallFunction|AdjustGhostTextSettings _structout)
  ;[1 1 1] Update server
  (if (Variables|ToolSetting|GetbServerSettingsInited)
    (CallFunction|SetTextSettingsOwningClient (Variables|ToolSetting|GetRunTimeSettings))))

(event Custom|Setting_SetColor
  (params (Color :type Linear%20Color%20Structure))
  ;[1 1 1] Settings (from widgets and onload)
  (bind _structout (Utilities|Struct|SetmembersinTextToolActorSettings (Variables|ToolSetting|GetRunTimeSettings) Color))
  (CallFunction|AdjustGhostTextSettings _structout)
  ;[1 1 1] Update server
  (if (Variables|ToolSetting|GetbServerSettingsInited)
    (CallFunction|SetTextSettingsOwningClient (Variables|ToolSetting|GetRunTimeSettings))))

(event Custom|Setting_SetSize
  (params (Value :type Float%20%28single-precision%29))
  ;[1 1 1] Settings (from widgets and onload)
  (bind _structout (Utilities|Struct|SetmembersinTextToolActorSettings (Variables|ToolSetting|GetRunTimeSettings) Value))
  (CallFunction|AdjustGhostTextSettings _structout)
  ;[1 1 1] Update server
  (if (Variables|ToolSetting|GetbServerSettingsInited)
    (CallFunction|SetTextSettingsOwningClient (Variables|ToolSetting|GetRunTimeSettings))))

(event Custom|Settings_TextChanged
  (params (Text :type String))
  ;[1 1 1] Settings (from widgets and onload)
  (bind _structout (Utilities|Struct|SetmembersinTextToolActorSettings (Variables|ToolSetting|GetRunTimeSettings) Text))
  (CallFunction|AdjustGhostTextSettings _structout)
  ;[1 1 1] Update server
  (if (Variables|ToolSetting|GetbServerSettingsInited)
    (CallFunction|SetTextSettingsOwningClient (Variables|ToolSetting|GetRunTimeSettings))))

(event Custom|Settings_AttachChanged
  (params (Attached :type Boolean))
  ;[1 1 1] Settings (from widgets and onload)
  (bind _structout (Utilities|Struct|SetmembersinTextToolActorSettings (Variables|ToolSetting|GetRunTimeSettings) Attached))
  (CallFunction|AdjustGhostTextSettings _structout)
  ;[1 1 1] Update server
  (if (Variables|ToolSetting|GetbServerSettingsInited)
    (CallFunction|SetTextSettingsOwningClient (Variables|ToolSetting|GetRunTimeSettings))))

(event Custom|SetTextSettingsOwningClient
  (params (Settings :type Text%20Tool%20Actor%20Settings%20Structure))
  ;[1 1 1] Replicate changes
  (CallFunction|SetTextSettingsServer Settings))

(event Custom|Settings_PhysicsChanged
  (params (Enabled :type Boolean))
  ;[1 1 1] Settings (from widgets and onload)
  (bind _structout (Utilities|Struct|SetmembersinTextToolActorSettings (Variables|ToolSetting|GetRunTimeSettings) Enabled))
  (CallFunction|AdjustGhostTextSettings _structout)
  ;[1 1 1] Update server
  (if (Variables|ToolSetting|GetbServerSettingsInited)
    (CallFunction|SetTextSettingsOwningClient (Variables|ToolSetting|GetRunTimeSettings))))

(event Custom|SetTextSettingsServer
  (params (Settings :type Text%20Tool%20Actor%20Settings%20Structure))
  ;[1 1 1] Replicate changes
  (Variables|ToolSetting|SetRunTimeSettings Settings))

(event Custom|InitSettings
  ;[1 1 1] Init / Load previous settings
  (bind _returnvalue (Class|KJModToolProxy|LoadToolSettings "TextToolSettings_10Nov20"))
  (Utilities|IsValid _returnvalue ; No save? use defaults
    (:Is%20Valid
      (bind _astext_tool_save_game_bp (Utilities|Casting|CastToTextToolSaveGameBP _returnvalue))
      (Utilities|FlowControl|Sequence
        (:then_0
          ;[1 1 1] Local Initial settings
          (CallFunction|SettingsTextChanged (Variables|/Game/CustomContent/UGC2281370083/Blueprints/TextTool/TextToolSaveGameBP.TextToolSaveGameBP_C|GetDefaultText _astext_tool_save_game_bp)))
        (:then_1
          (CallFunction|SettingSetSize (Variables|/Game/CustomContent/UGC2281370083/Blueprints/TextTool/TextToolSaveGameBP.TextToolSaveGameBP_C|GetSize _astext_tool_save_game_bp)))
        (:then_2
          (CallFunction|SettingSetColor (Variables|/Game/CustomContent/UGC2281370083/Blueprints/TextTool/TextToolSaveGameBP.TextToolSaveGameBP_C|GetColor _astext_tool_save_game_bp)))
        (:then_3
          (CallFunction|SettingSetZOffset (Variables|/Game/CustomContent/UGC2281370083/Blueprints/TextTool/TextToolSaveGameBP.TextToolSaveGameBP_C|GetZOffset _astext_tool_save_game_bp)))
        (:then_4
          (CallFunction|SettingsAttachChanged (Variables|/Game/CustomContent/UGC2281370083/Blueprints/TextTool/TextToolSaveGameBP.TextToolSaveGameBP_C|GetAttach _astext_tool_save_game_bp)))
        (:then_5
          (CallFunction|SettingsPhysicsChanged (Variables|/Game/CustomContent/UGC2281370083/Blueprints/TextTool/TextToolSaveGameBP.TextToolSaveGameBP_C|GetPhysicsEnabled _astext_tool_save_game_bp)))
        (:then_6
          ;;[1 1 1] Init settings server
          (CallFunction|SetTextSettingsOwningClient (Variables|ToolSetting|GetRunTimeSettings) :!label _label)
          (Variables|ToolSetting|SetbServerSettingsInited true))))
    (:Is%20Not%20Valid
      (goto _label))))

(fn ConstructionScript)

(fn CreateandShowToolsAssistInformation
  (Class|KJModToolProxy|ShowToolAssistUI)
  (Class|KJModToolProxy|SetToolAssistTitle "Text" "Text can be positioned, scaled and coloured")
  (Class|KJModToolProxy|ClearToolAssistFunctions)
  (bind _returnvalue (Class|KJModToolProxy|CreateToolAssistFunction "Add text to the selected point"))
  (Class|KJModToolProxy|SetToolAssistFunctionPrimaryDetails _returnvalue "LeftMouse"))

(fn CreateGhostText
  (bind _returnvalue (Game|GetPlayerCameraManager 0))
  (Class|KJModToolProxy|SpawnItem "/Game/CustomContent/UGC2281370083/Blueprints/TextTool/Prop/TextPropBP" (+ (Transformation|GetActorLocation _returnvalue) (* (Transformation|GetActorForwardVector _returnvalue) 5e+02)) "0, 0, 0" "1.000000,1.000000,1.000000"))

(fn ToolProxyGetToolSettingPanel
  (Utilities|IsValid (Variables|ToolSetting|GetToolSettingsWidget)
    (:Is%20Valid
      _)
    (:Is%20Not%20Valid
      (bind _returnvalue (UserInterface|CreateWidget "/Game/CustomContent/UGC2281370083/Blueprints/TextTool/Settings/TextToolSettingsWidgetBP.TextToolSettingsWidgetBP_C" (Game|GetPlayerController 0) self))
      (Default|CreatedEvent _returnvalue)
      (Variables|ToolSetting|SetToolSettingsWidget _returnvalue)))
  (return (Variables|ToolSetting|GetToolSettingsWidget)))

(fn OnRepSpawnedTextActor
  (bind _spawnedtextactor (Variables|Spawning|GetSpawnedTextActor))
  ;[1 1 1] If we're the owner then record the text creation in our history (for delete)
  (Utilities|IsLocallyControlled
    (:LocalControl
      (Utilities|IsValid _spawnedtextactor
        (:Is%20Valid
          (CallFunction|UpdateHistoryOwningClient _spawnedtextactor))))))