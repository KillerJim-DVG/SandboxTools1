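; Text prop for the TextTool that shows configurable world text, either as a ghost preview or as a stamped-down prop.
; Replicated Settings drive text, size and colour through OnRep, with optional attachment that sets collision and destroys the prop with its parent.
; Ghost edits are debounced on the owning client, then relayed through server to multicast.
; The box collider is sized from the text bounds for physgun interaction.
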(event Custom|AttachParentDestroyed
  (params (DestroyedActor :type Actor%20Object%20Reference))
  ;[1 1 1] When parent dies, we die..
  (Development|PrintString (Utilities|String|Append "Destroyed: " (Utilities|GetDisplayName DestroyedActor)))
  (Actor|DestroyActor))

(event Custom|SetGhostTextSettingsOwningClient
  (params (Settings :type Text%20Tool%20Actor%20Settings%20Structure))
  ;[1 1 1] GHOST TEXT - Set up correctly (this is shown prior to stamping down a real version)
  (Utilities|FlowControl|RetriggerableDelay 0.1) ; Stop flooding of network on lots of changes.. wait 100ms
  (CallFunction|SetGhostTextSettingsServer Settings))

(event Custom|SetGhostTextSettingsServer
  (params (Settings :type Text%20Tool%20Actor%20Settings%20Structure))
  ;[1 1 1] GHOST TEXT - Set up correctly (this is shown prior to stamping down a real version)
  (CallFunction|SetGhostTextSettingsMulticast Settings))

(event Custom|SetGhostTextSettingsMulticast
  (params (Settings :type Text%20Tool%20Actor%20Settings%20Structure))
  (bind (_text _size _colour) (Utilities|Struct|BreakTextToolActorSettings Settings))
  ;[1 1 1] GHOST TEXT - Set up correctly (this is shown prior to stamping down a real version)
  (Rendering|Components|TextRender|SetText (Variables|Default|GetTextRender) (Utilities|Text|ToText(String) _text))
  (Rendering|Components|TextRender|SetWorldSize (Variables|Default|GetTextRender) _size)
  (Rendering|Components|TextRender|SetTextRenderColor (Variables|Default|GetTextRender) (Math|Conversions|ToColor(LinearColor) _colour)))

(event Custom|RealiseSettings
  (params (Settings :type Text%20Tool%20Actor%20Settings%20Structure%20%28by%20ref%29))
  (bind (_text _size _colour _zoffset _attach _attachto _enablephysics) (Utilities|Struct|BreakTextToolActorSettings Settings))
  (bind _textrender (Variables|Default|GetTextRender))
  (bind _returnvalue (Class|TextRenderComponent|GetTextLocalSize _textrender))
  (bind (_x _y _z) (Math|Vector|BreakVector _returnvalue))
  ;[1 1 1] REALISE SETTINGS - Called via OnRep call
  (Rendering|Components|TextRender|SetText (Variables|Default|GetTextRender) (Utilities|Text|ToText(String) _text))
  (Rendering|Components|TextRender|SetWorldSize (Variables|Default|GetTextRender) _size)
  (Rendering|Components|TextRender|SetTextRenderColor (Variables|Default|GetTextRender) (Math|Conversions|ToColor(LinearColor) _colour))
  (if _attach
    (Utilities|IsValid _attachto
      (:Is%20Valid
        (Transformation|AttachActorToActor _attachto "None" "KeepWorld" "KeepWorld" "KeepWorld" true)
        (Game|BindEventtoOnDestroyed _attachto (delegate Custom|AttachParentDestroyed))
        (Collision|SetCollisionProfileName (Variables|Default|GetBox) (select _enablephysics "PhysicsActor" "NoCollision") true :!class /Script/Engine.PrimitiveComponent)
        ;[1 1 1] Ensure the collider (for physgun interactions) is sized exactly as the font/text
        (Utilities|FlowControl|Delay 0.1)
        (Components|Box|SetBoxExtent (Variables|Default|GetBox) (Math|Vector|MakeVector (Math|Float|Max(Float) _x 1.0) (Math|Float|Max(Float) _y 1.0) (Math|Float|Max(Float) _z 1.0)) true)))))

(fn ConstructionScript
  (bind _textrender (Variables|Default|GetTextRender))
  (bind _returnvalue (Class|TextRenderComponent|GetTextLocalSize _textrender))
  (bind (_x _y _z) (Math|Vector|BreakVector _returnvalue))
  (Components|Box|SetBoxExtent (Variables|Default|GetBox) (Math|Vector|MakeVector (Math|Float|Max(Float) _x 4.0) (Math|Float|Max(Float) _y 4.0) (Math|Float|Max(Float) _z 4.0)) true))

(fn OnRepSettings
  (CallFunction|RealiseSettings (Variables|Default|GetSettings)))