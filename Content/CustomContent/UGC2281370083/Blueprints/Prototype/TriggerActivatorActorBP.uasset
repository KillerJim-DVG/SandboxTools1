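; Test helper actor that fakes a player activating a target actor, so thrusters can be visually checked with Play in Editor.
; On BeginPlay, the authority starts a looping timer that toggles an active flag every couple of seconds.
; Each toggle prints the state and sends an activated or deactivated message to TargetActor.
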(event Custom|CustomEvent_0
  ;[0.2352 1 0] This little actor allows the thrusters to be tested by pressing play inside the editor; it just fakes a player activating the actor (used to make sure it was visually correct)
  (bind _output_get (Variables|Default|SetActiveFlag (not (Variables|Default|GetActiveFlag))))
  (if _output_get
    (Development|PrintString "+++ ACTIVATED")
    (Class|KJModTriggerInterface|Activated(Message) (Variables|Default|GetTargetActor))
    (else
      (Development|PrintString "--- DEACTIVATED")
      (Class|KJModTriggerInterface|Deactivated(Message) (Variables|Default|GetTargetActor)))))

(event EventBeginPlay
  ;[0.2352 1 0] This little actor allows the thrusters to be tested by pressing play inside the editor; it just fakes a player activating the actor (used to make sure it was visually correct)
  (Networking|SwitchHasAuthority
    (:Authority
      (bind _returnvalue (Utilities|Time|SetTimerbyEvent (delegate Custom|CustomEvent_0) 2.0 true)))))

(fn ConstructionScript)