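; Base camera prop that takes over the owning player's view when activated through a trigger interface.
; Activation disables the pawn camera and switches the view target to this actor with outgoing lock; deactivation re-enables the pawn camera.
; Each tick, it rotates to face the locked target component whenever one is valid.
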(event EventTick
  (params (DeltaSeconds :type Float%20%28single-precision%29))
  (bind _lockedtargetcomponent (Variables|Default|GetLockedTargetComponent))
  ;[1 1 1] EVENT TICK - Apply look at if required
  (if (Utilities|IsValid _lockedtargetcomponent)
    (Transformation|SetActorRotation (Math|Rotator|FindLookatRotation (Transformation|GetActorLocation) (Transformation|GetWorldLocation _lockedtargetcomponent)) true)))

(event EventActivated
  ;[1 1 1] Activation - TRIGGER INTERFACE
  (Utilities|IsValid (Variables|Default|GetOwningPlayerController)
    (:Is%20Valid
      (Class|KJModPlayerProxy|SetPawnCameraEnabled (Variables|Default|GetOwningPlayerController) false)
      (Game|Player|SetViewTargetwithBlend (Variables|Default|GetOwningPlayerController) self 0.0 "VTBlend_Linear" 0.0 true))))

(event EventDeactivated
  ;[1 1 1] Activation - TRIGGER INTERFACE
  (Utilities|IsValid (Variables|Default|GetOwningPlayerController)
    (:Is%20Valid
      (Class|KJModPlayerProxy|SetPawnCameraEnabled (Variables|Default|GetOwningPlayerController) true))))

(fn ConstructionScript)