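; Player tool that spawns a triggerable camera prop, either static or following a target.
; Tick traces from the pawn camera for a target; left click spawns the prop or locks it to that target, right click locks it to the pawn's camera.
; Saved trigger settings are realised for server-side spawning, where new cameras replace any sharing their key binding.
; Some wheel-named events remain, moving the prop and recording history.
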(event Custom|UpdateHistoryOwningClient
  (params (ObjectToAttach :type Actor%20Object%20Reference))
  ;[1 1 1] Update the history (to reflect last selection as most recent)
  (Class|KJModToolProxy|AddHistoryEntry (Utilities|Struct|MakeKJModToolHistoryItem ObjectToAttach "Removing wheel" "Wheel" "DeleteItem")))

(event Custom|SetWheelInformationOwningClient
  (params (Location :type Vector) (Visible :type Boolean) (TargetActor :type Actor%20Object%20Reference) (TargetComponent :type Primitive%20Component%20Object%20Reference) (Rotation :type Rotator))
  (bind _spawnedcameraprop (Variables|Spawning|GetSpawnedCameraProp))
  ;[1 1 1] Update ghost wheel position and settings information (local and remote)
  (CallFunction|SetWheelInformationServer Location Visible TargetActor TargetComponent Rotation)
  (Utilities|IsValid _spawnedcameraprop ; may not be replicated yet
    (:Is%20Valid
      (Transformation|SetActorLocation _spawnedcameraprop Location false true)
      (Transformation|SetActorRotation _spawnedcameraprop Rotation true)
      (Rendering|SetActorHiddenInGame _spawnedcameraprop (not Visible)))))

(event Custom|SetWheelInformationServer
  (params (Location :type Vector) (Visible :type Boolean) (TargetActor :type Actor%20Object%20Reference) (TargetComponent :type Primitive%20Component%20Object%20Reference) (Rotation :type Rotator))
  (bind _spawnedcameraprop (Variables|Spawning|GetSpawnedCameraProp))
  ;[1 1 1] Update ghost wheel position and settings information (local and remote)
  (Utilities|Struct|SetmembersinCameraToolActorSettings (Variables|ToolSetting|GetSettings) TargetActor TargetComponent)
  (Utilities|IsValid _spawnedcameraprop ; Is null when switching lamp's
    (:Is%20Valid
      (Transformation|SetActorLocation _spawnedcameraprop Location false true)
      (Transformation|SetActorRotation _spawnedcameraprop Rotation true)
      (Rendering|SetActorHiddenInGame _spawnedcameraprop (not Visible)))))

(event EventBeginPlay
  ;[0.9593 1 0.1335] BEGIN PLAY EVENT
  (Networking|SwitchHasAuthority
    (:Authority
      ;;[1 1 1] Listen server?
      (if (not (Networking|IsDedicatedServer))
        (Utilities|FlowControl|Sequence
          (:then_1
            ;;[1 1 1] If local controlled; init once..
            (Utilities|IsLocallyControlled :!label _label
              (:LocalControl
                (CallFunction|NotifyOwnerOfInstantiation)
                (if (not (Variables|Initialisation|GetInitialised))
                  (Variables|Initialisation|SetInitialised true)
                  ;;[1 1 1] Reload settings
                  (CallFunction|CreateandShowToolsAssistInformation)
                  (CallFunction|InitSettings)
                  (CallFunction|InitTriggerSettings))))))))
    (:Remote
      (goto _label))))

(event EventTick
  (params (DeltaSeconds :type Float%20%28single-precision%29))
  ;[1 1 1] EVENT TICK
  (|CallParentFunction DeltaSeconds)
  (Networking|SwitchHasAuthority
    (:Authority
      ;;[1 1 1] Listen server?
      (if (not (Networking|IsDedicatedServer))
        ;;[1 1 1] Handle MOUSE SELECTION POINT
        (bind _returnvalue (Class|KJModToolProxy|GetPawnCameraComponent :!label _label))
        (bind (_outhit _returnvalue_2) (Collision|LineTraceByChannel (Transformation|GetWorldLocation _returnvalue) (+ (Transformation|GetWorldLocation _returnvalue) (* (Math|Vector|GetForwardVector _returnvalue) 1.5e+04)) "TraceTypeQuery1" true (Utilities|Array|MakeArray (Game|Player|GetPlayerPawn 0)) "None"))
        (if _returnvalue_2
          (if (.bBlockingHit (Collision|BreakHitResult _outhit))
            (Variables|Spawning|SetLookAtTargetComplonent (.HitComponent (Collision|BreakHitResult _outhit)))
            (else
              (Variables|Spawning|SetLookAtTargetComplonent 0 :!label _label_2)))
          (else
            (goto _label_2)))))
    (:Remote
      (goto _label))))

(event EventToolProxyItemSpawned
  (params (spawnedActor :type Actor%20Object%20Reference))
  ;[1 1 1] (interface) Item Spawned - From Pawn
  (bind _ascamera_base_prop_bp (Utilities|Casting|CastToCameraBasePropBP spawnedActor)
    (:then
      (Utilities|FlowControl|Sequence
        (:then_0
          ;;[1 1 1] Remove any cameras that have our binding..
          (bind _outactors (Actor|GetAllActorsOfClass "/Game/CustomContent/UGC2281370083/Blueprints/Camera/Props/CameraBasePropBP.CameraBasePropBP_C"))
          (for _array_element _outactors
            (if (== (Variables|Default|GetTriggerKey) (Variables|/Game/CustomContent/UGC2281370083/Blueprints/Camera/Props/CameraBasePropBP.CameraBasePropBP_C|GetBindKey _array_element))
              (Actor|DestroyActor _array_element))))
        (:then_1
          (bind _output_get (Variables|Spawning|SetSpawnedCameraProp _ascamera_base_prop_bp))
          (Variables|/Game/CustomContent/UGC2281370083/Blueprints/Camera/Props/CameraBasePropBP.CameraBasePropBP_C|SetOwningPlayerController _output_get (.AsPlayer%20Controller (Utilities|Casting|CastToPlayerController (Pawn|GetController (.AsPawn (Utilities|Casting|CastToPawn (Components|GetOwner)))))))
          ;;[1 0.2686 0.01696 1 14] Record what key binds to this camera; so we can delete it if a new camera with the same bind appears
          (if (Variables|Default|GetTriggerable)
            (Variables|/Game/CustomContent/UGC2281370083/Blueprints/Camera/Props/CameraBasePropBP.CameraBasePropBP_C|SetBindKey _output_get (Variables|Default|GetTriggerKey)))
          (Class|KJModToolProxy|RegisterTriggerActor _output_get)
          (Class|KJModToolProxy|SetTrigger _output_get (Variables|Default|GetTriggerable) (Variables|Default|GetTriggerType) (Variables|Default|GetTriggerKey) (Variables|Default|GetTriggerEventName))
          (Class|KJModToolProxy|PlayToolSoundEffect "ToolSpawnSound" true))))
    (:CastFailed
      (|CallParentFunction spawnedActor))))

(event Custom|LockTargetToProp
  (params (LockedTargetComponent :type Scene%20Component%20Object%20Reference))
  ;[1 1 1] LEFT/RIGHT MOUSE - Drop or freeze if anything on tool
  ;;[1 1 1] Left - Attempt Grab or Release any object
  ;;;[1 1 1] Call on server; tell camera prop to look at component (replicated)
  (Variables|/Game/CustomContent/UGC2281370083/Blueprints/Camera/Props/CameraBasePropBP.CameraBasePropBP_C|SetLockedTargetComponent (Variables|Spawning|GetSpawnedCameraProp) LockedTargetComponent))

(event EventToolProxySecondaryMouseClick
  (params (pressed :type Boolean))
  ;[1 1 1] LEFT/RIGHT MOUSE - Drop or freeze if anything on tool
  ;;[1 1 1] Left - Attempt Grab or Release any object
  (if pressed ; Pressed?
    (Utilities|IsValid (Variables|Spawning|GetLookAtTargetComplonent)
      (:Is%20Valid
        (Class|KJModToolProxy|PlayToolSoundEffect "ToolSelectionSound" true)
        (bind _returnvalue (Class|KJModToolProxy|GetPawnCameraComponent))
        (CallFunction|LockTargettoProp _returnvalue)))))

(event EventToolProxyPrimaryMouseClick
  (params (pressed :type Boolean))
  ;[1 1 1] LEFT/RIGHT MOUSE - Drop or freeze if anything on tool
  ;;[1 1 1] Left - Attempt Grab or Release any object
  (if pressed ; Pressed?
    (Utilities|IsValid (Variables|Spawning|GetSpawnedCameraProp)
      (:Is%20Valid
        (Class|KJModToolProxy|PlayToolSoundEffect "ToolSelectionSound" true)
        (CallFunction|LockTargettoProp (Variables|Spawning|GetLookAtTargetComplonent)))
      (:Is%20Not%20Valid
        (bind _returnvalue (Class|KJModToolProxy|GetPawnCameraComponent))
        (Class|KJModToolProxy|SpawnItem "/Game/CustomContent/UGC2281370083/Blueprints/Camera/Props/CameraBasePropBP" (Transformation|GetWorldLocation _returnvalue) (Transformation|GetWorldRotation _returnvalue) "1.000000,1.000000,1.000000")
        (Variables|Default|SetRespawnDelayTimeout 0.5)
        (Class|KJModToolProxy|PlayToolSoundEffect "ToolSpawnSound" true)))))

(event Custom|TriggerWidgetSettingsChanged
  ;[1 1 1] Trigger widget has said a change has been saved, reload it
  (CallFunction|InitTriggerSettings))

(event Custom|InitSettings
  ;[1 1 1] LOAD / REALISE TOOL SPECIFIC SETTINGS
)

(event Custom|RealiseSettings
  (params (Triggerable :type Boolean) (Selection :type Integer) (TriggerKey :type Input%20Chord%20Structure) (TriggerEventName :type String))
  ;[1 1 1] SERVER LOAD - These settings are used server side
  (Utilities|FlowControl|Sequence
    (:then_0
      (Variables|Default|SetTriggerable Triggerable))
    (:then_1
      (switch int Selection
        (:0
          (Variables|Default|SetTriggerType "KeyHeldTrigger"))
        (:1
          (Variables|Default|SetTriggerType "KeyPressToggle"))
        (:2
          (Variables|Default|SetTriggerType "NamedEventToggleTrigger"))))
    (:then_2
      (Variables|Default|SetTriggerKey TriggerKey))
    (:then_3
      (Variables|Default|SetTriggerEventName TriggerEventName))))

(event Custom|InitTriggerSettings
  ;[1 1 1] LOAD BASE TRIGGER SETTINGS - Grab the base settings and transfer to server (as it spawns the wheel and needs them there)
  (bind _returnvalue (Class|KJModToolProxy|LoadToolSettings "CameraBaseSettings"))
  (Utilities|IsValid _returnvalue
    (:Is%20Valid
      (bind _asbase_tool_save_game_bp (Utilities|Casting|CastToBaseToolSaveGameBP _returnvalue))
      (CallFunction|RealiseSettings (Variables|/Game/CustomContent/UGC2281370083/Blueprints/BaseToolSaveGameBP.BaseToolSaveGameBP_C|GetTriggerable _asbase_tool_save_game_bp) (Variables|/Game/CustomContent/UGC2281370083/Blueprints/BaseToolSaveGameBP.BaseToolSaveGameBP_C|GetTriggerType _asbase_tool_save_game_bp) (Variables|/Game/CustomContent/UGC2281370083/Blueprints/BaseToolSaveGameBP.BaseToolSaveGameBP_C|GetTriggerKey _asbase_tool_save_game_bp) (Variables|/Game/CustomContent/UGC2281370083/Blueprints/BaseToolSaveGameBP.BaseToolSaveGameBP_C|GetTriggerEventName _asbase_tool_save_game_bp)))))

(fn ConstructionScript)

(fn CreateandShowToolsAssistInformation
  (Class|KJModToolProxy|ShowToolAssistUI)
  (Class|KJModToolProxy|SetToolAssistTitle "Camera" "A triggerable camera that's static or follows props")
  (Class|KJModToolProxy|ClearToolAssistFunctions)
  (Utilities|FlowControl|Sequence
    (:then_0
      (bind _returnvalue (Class|KJModToolProxy|CreateToolAssistFunction "Spawn the camera, then lock to selected prop"))
      (Class|KJModToolProxy|SetToolAssistFunctionPrimaryDetails _returnvalue "LeftMouse"))
    (:then_1
      (bind _returnvalue_2 (Class|KJModToolProxy|CreateToolAssistFunction "Toggle following the player"))
      (Class|KJModToolProxy|SetToolAssistFunctionPrimaryDetails _returnvalue_2 "RightMouse"))))

(fn ToolProxyGetToolSettingPanel
  (Utilities|IsValid (Variables|ToolSetting|GetToolSettingsWidget)
    (:Is%20Valid
      _)
    (:Is%20Not%20Valid
      (bind _returnvalue (UserInterface|CreateWidget "/Game/CustomContent/UGC2281370083/Blueprints/Camera/Settings/CameraToolSettingsWidgetBP.CameraToolSettingsWidgetBP_C" (Game|GetPlayerController 0) self))
      (Default|CreatedEvent _returnvalue)
      (bind _output_get (Variables|ToolSetting|SetToolSettingsWidget _returnvalue))
      ;[1 1 1] We want to listen to changes from the trigger widget part
      (EventDispatchers|BindEventtoTriggerWidgetUpdated (Variables|/Game/CustomContent/UGC2281370083/Blueprints/Camera/Settings/CameraToolSettingsWidgetBP.CameraToolSettingsWidgetBP_C|GetBaseTriggerWidgetBP _output_get) (EventDispatchers|CreateEvent :!event Custom|TriggerWidgetSettingsChanged))))
  (return (Variables|ToolSetting|GetToolSettingsWidget)))

(fn OnRepSpawnedCameraProp
  (bind _spawnedcameraprop (Variables|Spawning|GetSpawnedCameraProp))
  ;[1 1 1] If we're the owner then record the Wheels creation in our history (for delete)
  (Utilities|IsLocallyControlled
    (:LocalControl
      (Utilities|IsValid _spawnedcameraprop
        (:Is%20Valid
          (CallFunction|UpdateHistoryOwningClient _spawnedcameraprop))))))