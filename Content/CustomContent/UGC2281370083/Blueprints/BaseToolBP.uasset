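; Base Blueprint for sandbox tools, providing shared item spawning, deletion, freezing and gravity toggling.
; A replicated SpawnedActor's OnRep records history for the locally controlled owner, and a custom delete key pops the latest entry and destroys that actor.
; Repeat-last-action respawns the last asset in front of the camera, with a Tick-driven cooldown against spamming.
; Owning-client events show player messages, then pass physics changes and destruction to server events.
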(event Custom|SetGravityEnabledServer
  (params (ParentActor :type Actor%20Object%20Reference))
  ;[1 1 1] GRAVITY (server-side)
  (Utilities|IsValid ParentActor
    (:Is%20Valid
      (for _array_element (Actor|GetComponentsByClass ParentActor "/Script/Engine.PrimitiveComponent")
        (Physics|SetEnableGravity _array_element (not (Class|PrimitiveComponent|IsGravityEnabled _array_element)))))))

(event Custom|ToggleGravityOwningClient
  (params (ParentActor :type Actor%20Object%20Reference))
  ;[1 1 1] GRAVITY (server-side)
  (if (Physics|IsSimulatingPhysics (Actor|GetComponentbyClass ParentActor "/Script/Engine.PrimitiveComponent") "None")
    (CallFunction|SetGravityEnabledServer ParentActor)
    (CallFunction|ShowMessagetoLocalPlayer "Gravity toggled on item" 2.0 false)
    (else
      (CallFunction|ShowMessagetoLocalPlayer "Can't toggle gravity, item frozen" 2.0 false))))

(event Custom|NotifyOwnerOfInstantiation
  ;[1 1 1] Call by a tool to tell the local client that it's active (registers settings widgets, etc.)
  (Class|KJModToolProxy|RegisterToolLocally))

(event Custom|BaseTool%20Delete%20Object
  ;[1 1 1] DELETE - If child doesn't inherit we just delete from history..
  (bind _actor (Utilities|GetLastActorfromHistory)
    (:Out
      (Utilities|IsValid _actor ; Nothing grabbed? or last one deleted?
        (:Is%20Valid
          (bind (_actor_2 _struct) (Utilities|GetandRemoveLastActorfromHistory)
            (:Out
              (CallFunction|DeleteContainerOwningClient _actor_2)
              (CallFunction|ShowMessagetoLocalPlayer (Utilities|String|Append "Removing " (.operationName (Utilities|Struct|BreakKJModToolHistoryItem _struct)) " by tool " (.toolName (Utilities|Struct|BreakKJModToolHistoryItem _struct))) 1.0 true))))
        (:Is%20Not%20Valid
          (CallFunction|ShowMessagetoLocalPlayer "Cannot delete, nothing left to delete!" 2.0 false))))))

(event Custom|ToggleFreezeStateOwningClient
  (params (ParentActor :type Actor%20Object%20Reference))
  (bind _returnvalue (Actor|GetComponentbyClass ParentActor "/Script/Engine.PrimitiveComponent"))
  (bind _returnvalue_2 (Physics|IsSimulatingPhysics _returnvalue "None"))
  (bind _returnvalue_3 (not _returnvalue_2))
  ;[1 1 1] Freeze (server-side)
  (if _returnvalue_3 ; User OP first, as in SP the code runs immediately inverting this branch
    (CallFunction|ShowMessagetoLocalPlayer "Item released" 2.0 false)
    (else
      (CallFunction|ShowMessagetoLocalPlayer "Item frozen" 2.0 false)))
  (CallFunction|SetFreezeStateServer ParentActor _returnvalue_3))

(event Custom|SetFreezeStateServer
  (params (ParentActor :type Actor%20Object%20Reference) (Unfreeze :type Boolean))
  ;[1 1 1] Freeze (server-side)
  (Utilities|IsValid ParentActor
    (:Is%20Valid
      (for _array_element (Actor|GetComponentsByClass ParentActor "/Script/Engine.PrimitiveComponent")
        (Physics|SetSimulatePhysics _array_element Unfreeze)))))

(event EventToolProxyRepeatLastAction
  ;[1 1 1] R KEY - respawn last item
  (if (and (<= (Variables|Respawning|GetRespawnDelayTimeout) 0.0) (Utilities|Enum|NotEqual(Enum) (Variables|Respawning|GetLastKnownAssetPakPath) ""))
    (Class|KJModToolProxyInterface|ToolProxySpawnItem (Variables|Respawning|GetLastKnownAssetPakPath))
    (Variables|Respawning|SetRespawnDelayTimeout 0.5)))

(event EventToolProxySpawnItem
  (params (assetPath :type String))
  (bind _returnvalue (Game|GetPlayerCameraManager 0))
  ;[1 1 1] SPAWN ITEM (Used by tools that don't want to support this natively)
  (Class|KJModToolProxy|SpawnItem assetPath (+ (Transformation|GetActorLocation _returnvalue) (* (Transformation|GetActorForwardVector _returnvalue) 5e+02)) "0, 0, 0" "1.000000,1.000000,1.000000")
  (Variables|Respawning|SetLastKnownAssetPakPath assetPath))

(event EventTick
  (params (DeltaSeconds :type Float%20%28single-precision%29))
  ;[1 1 1] Time out the respawn logic (to stop spamming)
  (if (> (Variables|Respawning|GetRespawnDelayTimeout) 0.0)
    (Variables|Respawning|SetRespawnDelayTimeout (- (Variables|Respawning|GetRespawnDelayTimeout) (Utilities|Time|GetWorldDeltaSeconds)))))

(event EventToolProxyItemSpawned
  (params (spawnedActor :type Actor%20Object%20Reference))
  ;[1 1 1] Item was spawned (server) - we set the replicated variable; so the remote z
  (Variables|Default|SetSpawnedActor spawnedActor))

(event EventToolProxyCustomActionPressed
  (params (cookie :type Integer) (pressed :type Boolean))
  ;[1 1 1] CUSTOM ACTIONS (KEY)
  (if (== cookie 1)
    (CallFunction|BaseToolDeleteObject)))

(event EventBeginPlay
  ;[1 1 1] CUSTOM ACTIONS (KEY)
  (Utilities|HandleClientServerLogic
    (:ClientLogic
      (Class|KJModToolProxy|SetCustomAction "Z" "Physgun_Delete" "Delete the next item in the spawned (or touched, depending on settings) history list" 1))))

(event Custom|DeleteContainerOwningClient
  (params (Actor :type Actor%20Object%20Reference))
  ;[1 1 1] Delete item - server side
  (CallFunction|DeleteContainerServer Actor))

(event Custom|DeleteContainerServer
  (params (Actor :type Actor%20Object%20Reference))
  ;[1 1 1] Delete item - server side
  (Actor|DestroyActor Actor))

(fn ConstructionScript)

(fn ShowMessagetoLocalPlayer
  (params (Message :type String) (TTL :type Float%20%28single-precision%29) (AllowDuplicates :type Boolean) (Texture :type Texture%202D%20Object%20Reference))
  (Class|KJModToolProxy|ShowMessage Message TTL AllowDuplicates Texture))

(fn OnRepSpawnedActor
  ;[1 1 1] Spawned Actor Replicated - Executed everywhere (just in case you want to know) but as the "owning" player we want to record history
  (bind _ascharacter (Utilities|Casting|CastToCharacter (Components|GetOwner)))
  (if (Pawn|IsLocallyControlled _ascharacter)
    (Class|KJModToolProxy|AddHistoryEntry (Utilities|Struct|MakeKJModToolHistoryItem (Variables|Default|GetSpawnedActor) "" (Variables|Default|GetToolName) "DeleteItem"))))