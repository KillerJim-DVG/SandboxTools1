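; Short-lived thruster prop that briefly flashes arrow indicators to show a forward or reverse direction.
; On clients, it creates dynamic materials for the front and back markers and animates their Alpha with a timeline.
; One of two timelines, chosen by ForwardDirection, drives the roll of the back indicator only.
; The server handles cleanup, destroying the actor after a short fixed delay.
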(event Custom|RotateArrows
  (if (Variables|Default|GetForwardDirection)
    (bind _newtrack_0 (Timeline|Timeline_0 PlayFromStart)
      (:Update
        (Transformation|SetRelativeRotation (Variables|Default|GetDirectionIndicator_Back) (Math|Rotator|MakeRotator _newtrack_0 0.0 0.0) false false)))
    (else
      (bind _newtrack_0_2 (Timeline|Timeline_1 PlayFromStart)
        (:Update
          (Transformation|SetRelativeRotation (Variables|Default|GetDirectionIndicator_Back) (Math|Rotator|MakeRotator _newtrack_0_2 0.0 0.0) false false))))))

(event Custom|FlashArrows
  (bind _newtrack_0 (Timeline|FlashUpDown PlayFromStart)
    (:Update
      (Rendering|Material|SetScalarParameterValue (Variables|Default|GetBackDynamicMaterialInstance) "Alpha" _newtrack_0 :!class /Script/Engine.MaterialInstanceDynamic)
      (Rendering|Material|SetScalarParameterValue (Variables|Default|GetFrontDynamicMaterialInstance) "Alpha" _newtrack_0 :!class /Script/Engine.MaterialInstanceDynamic))))

(event EventBeginPlay
  (Utilities|HandleClientServerLogic
    (:ServerLogic
      (Utilities|FlowControl|Delay 1.2)
      (Actor|DestroyActor))
    (:ClientLogic
      (CallFunction|CreateDynamicArryowMaterial)
      (CallFunction|FlashArrows)
      (CallFunction|RotateArrows))))

(fn ConstructionScript)

(fn CreateDynamicArryowMaterial
  (Utilities|FlowControl|Sequence
    (:then_0
      (bind _returnvalue (Rendering|Material|CreateDynamicMaterialInstance (Variables|Default|GetDirectionIndicator_Back) 0 "/Game/CustomContent/UGC2281370083/Blueprints/Thrusters/Models/DirectionMarker/DirectionMarkerMat.DirectionMarkerMat" "None" :!class /Script/Engine.PrimitiveComponent))
      (bind _output_get (Variables|Default|SetBackDynamicMaterialInstance _returnvalue))
      (Rendering|Material|SetScalarParameterValue _output_get "Alpha" 0.0 :!class /Script/Engine.MaterialInstanceDynamic))
    (:then_1
      (bind _returnvalue_2 (Rendering|Material|CreateDynamicMaterialInstance (Variables|Default|GetDirectionIndicator_Front) 0 "/Game/CustomContent/UGC2281370083/Blueprints/Thrusters/Models/DirectionMarker/DirectionMarkerMat.DirectionMarkerMat" "None" :!class /Script/Engine.PrimitiveComponent))
      (bind _output_get_2 (Variables|Default|SetFrontDynamicMaterialInstance _returnvalue_2))
      (Rendering|Material|SetScalarParameterValue _output_get_2 "Alpha" 0.0 :!class /Script/Engine.MaterialInstanceDynamic))))