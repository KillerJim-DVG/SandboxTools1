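; Base thruster prop that a tool attaches to another component, simulating physics and pushing through a PhysicsThruster with torque-scaled strength.
; Attachment configures the physics constraint, and a looping server timer destroys the thruster if its connected actor becomes invalid.
; Trigger interface events set Active, whose OnRep toggles thrust and client-side staged rocket audio, particles and timeline-driven light flicker.
; Ghost-preview settings and replicated attach logic are unfinished or unused.
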(event Custom|SetThrusterAttachedActor
  (params (Settings :type Thruster%20Tool%20Actor%20Settings%20Structure))
  ;[1 1 1] SERVER - Attach to actor (spawn physical constraint)
  (CallFunction|SetThrusterAttachment Settings))

(event Custom|SetLightActive
  (params (Active :type Boolean))
  ;[1 1 1] Lighting Flicker with on/off handling
  (if Active
    (Rendering|SetVisibility (Variables|Default|GetSpotLight) true false)
    (Utilities|FlowControl|Sequence
      (:then_0
        (bind _newtrack_0 (Timeline|Flicker PlayFromStart)
          (:Update
            (Rendering|Components|Light|SetIntensity (Variables|Default|GetSpotLight) (* _newtrack_0 5e+05)))))
      (:then_1
        (bind _newtrack_0_2 (Timeline|Timeline_0 Stop)
          (:Update
            (Rendering|Components|Light|SetIntensity (Variables|Default|GetSpotLight) (* _newtrack_0_2 5e+05)))
          (:Finished
            (Rendering|SetVisibility (Variables|Default|GetSpotLight) false false)))))
    (else
      (Utilities|FlowControl|Sequence
        (:then_0
          (Timeline|Flicker Stop))
        (:then_1
          (Timeline|Timeline_0 PlayFromStart))))))

(event Custom|VisuallyActiveThruster
  (bind _audio (Variables|Default|GetAudio))
  ;[1 1 1] Active/Deactivate Visuals + Sounds
  (bind _returnvalue (Audio|SpawnSoundAttached "/Game/CustomContent/UGC2281370083/Blueprints/Thrusters/Sounds/RocketStartCue.RocketStartCue" (Variables|Default|GetAudio) "None" "0, 0, 0" "0, 0, 0" "SnapToTarget" false 1.0 1.0 0.0 0 0))
  (Variables|Default|SetInitialAudioCue _returnvalue)
  (Utilities|FlowControl|Delay 0.2)
  (if (Variables|Default|GetbActive)
    (Components|Activation|Deactivate (Variables|Default|GetCoolDownParticleSystem))
    (Components|Activation|SetActive (Variables|Default|GetParticleSystem) true true)
    (Components|Activation|SetActive (Variables|Default|GetParticleSystem1) true true)
    (CallFunction|SetLightActive true)
    (Utilities|FlowControl|RetriggerableDelay 1.8)
    (if (Variables|Default|GetbActive)
      (Audio|Components|Audio|SetSound _audio "/Game/CustomContent/UGC2281370083/Blueprints/Thrusters/Sounds/RocketLoopCue.RocketLoopCue")
      (Audio|Components|Audio|Play _audio 0.0)
      (Utilities|IsValid (Variables|Default|GetInitialAudioCue)
        (:Is%20Valid
          (Components|DestroyComponent (Variables|Default|GetInitialAudioCue)))))))

(event Custom|SetGhostThrusterSettingsOwningClient
  (params (Settings :type Thruster%20Tool%20Actor%20Settings%20Structure))
  ;[1 1 1] GHOST THRUSTER - Updating any parameters (run-time) - Technically a wheel only changes type at run-time but we keep it as example code
  (Utilities|FlowControl|RetriggerableDelay 0.1) ; Stop flooding of network on lots of changes.. wait 100ms
)

(event Custom|EnsureConnectionIsValid
  ;[1 1 1] If conected to something, make sure it exists or delete ourselves
  (Networking|SwitchHasAuthority
    (:Authority
      (Utilities|Time|SetTimerbyEvent (delegate Custom|ConnectionCheck) 0.1 true))))

(event Custom|ConnectionCheck
  ;[1 1 1] If conected to something, make sure it exists or delete ourselves
  (Utilities|IsValid (Variables|Default|GetConnectedActor)
    (:Is%20Not%20Valid
      (Actor|DestroyActor))))

(event Custom|SetGhostThrusterSettingsServer
  (params (Settings :type Thruster%20Tool%20Actor%20Settings%20Structure))
  ;[1 1 1] GHOST THRUSTER - Updating any parameters (run-time) - Technically a wheel only changes type at run-time but we keep it as example code
)

(event Custom|VisuallyDeactiveThruster
  (bind _audio (Variables|Default|GetAudio))
  ;[1 1 1] Active/Deactivate Visuals + Sounds
  (Audio|Components|Audio|Stop _audio)
  (Audio|Components|Audio|SetSound _audio "/Game/CustomContent/UGC2281370083/Blueprints/Thrusters/Sounds/RocketEndCue.RocketEndCue")
  (Audio|Components|Audio|Play _audio 0.0)
  (Components|Activation|Deactivate (Variables|Default|GetParticleSystem))
  (Components|Activation|Deactivate (Variables|Default|GetParticleSystem1))
  (Utilities|IsValid (Variables|Default|GetInitialAudioCue)
    (:Is%20Valid
      (Components|DestroyComponent (Variables|Default|GetInitialAudioCue)))
    (:Is%20Not%20Valid
      _))
  (Components|Activation|SetActive (Variables|Default|GetCoolDownParticleSystem) true true)
  (CallFunction|SetLightActive false))

(event Custom|SetThrusterAttachment
  (params (Settings :type Thruster%20Tool%20Actor%20Settings%20Structure))
  (bind (_connectedactor _connectedcomponent _torque _forcelimit _friction _nocollision) (Utilities|Struct|BreakThrusterToolActorSettings Settings))
  ;[1 0.8798 0.3503] MULTICAST - Set up constraint
  (Variables|Default|SetConnectedActor _connectedactor)
  (Variables|Default|SetConnectedComponent _connectedcomponent)
  (Variables|Default|SetTorque _torque)
  (CallFunction|EnsureConnectionIsValid)
  (Collision|SetCollisionProfileName (Variables|Default|GetThrusterMesh) "PhysicsActor" true :!class /Script/Engine.PrimitiveComponent)
  (Physics|SetSimulatePhysics (Variables|Default|GetThrusterMesh) true)
  (Class|PhysicsConstraintComponent|SetConstrainedComponents (Variables|Default|GetPhysicsConstraint) (Variables|Default|GetThrusterMesh) "None" (Variables|Default|GetConnectedComponent) "None")
  (Class|PhysicsConstraintComponent|SetDisableCollision (Variables|Default|GetPhysicsConstraint) _nocollision)
  (Variables|/Script/Engine.PhysicsThrusterComponent|SetThrustStrength (Variables|Default|GetPhysicsThruster) (* 500000 (Variables|Default|GetTorque))))

(event EventTick
  (params (DeltaSeconds :type Float%20%28single-precision%29))
  ;[1 1 1] EVENT TICK - Nothing to do (disabled in class settings)
)

(event EventActivated
  ;[1 1 1] Activation - TRIGGER INTERFACE
  (Variables|Default|SetbActive true))

(event EventDeactivated
  ;[1 1 1] Activation - TRIGGER INTERFACE
  (Variables|Default|SetbActive false))

(event EventBeginPlay
  ;[1 1 1] BEGIN PLAY - Should ghosted version..
)

(fn ConstructionScript)

(fn StoreBaseMaterialsandGhost
  (bind _thrustermesh (Variables|Default|GetThrusterMesh))
  (bind _returnvalue (Rendering|Material|GetMaterials _thrustermesh))
  (Variables|BaseMaterials|SetBaseMaterials _returnvalue)
  (for (_ _array_index) _returnvalue
    (Rendering|Material|CreateDynamicMaterialInstance (Variables|Default|GetThrusterMesh) _array_index "/Game/CustomContent/UGC2281370083/Blueprints/Thrusters/Props/ThrusterOutlineMat.ThrusterOutlineMat" "None" :!class /Script/Engine.PrimitiveComponent)))

(fn OnRepConnectedComponent
  (CallFunction|AttemptReplicatedAttach))

(fn AttemptReplicatedAttach
  ;[1 1 1] Not used
  (if (Math|Boolean|ANDBoolean (Utilities|IsValid (Variables|Default|GetPhysicsConstraint)) (Utilities|IsValid (Variables|Default|GetConnectedComponent)) (not (Ability|HasAuthority)))
    _))

(fn OnRepBActive
  (if (Variables|Default|GetbActive)
    (Components|Activation|SetActive (Variables|Default|GetPhysicsThruster) true true)
    (Utilities|HandleClientServerLogic
      (:ClientLogic
        (CallFunction|VisuallyActiveThruster)))
    (else
      (Components|Activation|SetActive (Variables|Default|GetPhysicsThruster) false true)
      (Utilities|HandleClientServerLogic
        (:ClientLogic
          (CallFunction|VisuallyDeactiveThruster))))))