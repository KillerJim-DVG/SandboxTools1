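; Player tool that joins two different actors with a rope, using two left clicks to pick the anchor points.
; On the controlling client, Tick traces from the camera to place a selection marker, mirrored to the server.
; Clicks check ownership, then the server spawns BuildARopeBP using settings synced from a widget or save game.
; A RepNotify on the spawned rope records it in the owner's tool history for deletion.
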(event Custom|UpdateHistoryOwningClient
  (params (ObjectToAttach :type Actor%20Object%20Reference))
  ;[1 1 1] Update the history (to reflect last selection as most recent)
  (Class|KJModToolProxy|AddHistoryEntry (Utilities|Struct|MakeKJModToolHistoryItem ObjectToAttach "rope" "Rope" "DeleteItem")))

(event Custom|SetRopeTargetOwningClient
  (params (Location :type Vector) (Visible :type Boolean) (Rotation :type Rotator))
  (bind _selectiontargetpointeractor (Variables|Targeting|GetSelectionTargetPointerActor))
  ;[1 1 1] Update target position
  (CallFunction|SetRopeTargetServer Location Visible Rotation)
  (Utilities|IsValid _selectiontargetpointeractor ; may not be replicated yet
    (:Is%20Valid
      (Transformation|SetActorLocation _selectiontargetpointeractor Location false true)
      (Transformation|SetActorRotation _selectiontargetpointeractor Rotation true)
      (Rendering|SetActorHiddenInGame _selectiontargetpointeractor (not Visible)))))

(event Custom|SetRopeTargetServer
  (params (Location :type Vector) (Visible :type Boolean) (Rotation :type Rotator))
  (bind _selectiontargetpointeractor (Variables|Targeting|GetSelectionTargetPointerActor))
  ;[1 1 1] Update target position
  (Utilities|IsValid _selectiontargetpointeractor ; Is null when switching lamp's
    (:Is%20Valid
      (Transformation|SetActorLocation _selectiontargetpointeractor Location false true)
      (Transformation|SetActorRotation _selectiontargetpointeractor Rotation true)
      (Rendering|SetActorHiddenInGame _selectiontargetpointeractor (not Visible)))))

(event EventDestroyed
  (bind _selectiontargetpointeractor (Variables|Targeting|GetSelectionTargetPointerActor))
  ;[1 1 1] DESTROYED - remove selection marker
  (Utilities|IsValid _selectiontargetpointeractor
    (:Is%20Valid
      (Actor|DestroyActor _selectiontargetpointeractor))))

(event EventBeginPlay
  ;[0.9593 1 0.1335] BEGIN PLAY EVENT
  (Networking|SwitchHasAuthority
    (:Authority
      ;;[1 1 1] Listen server?
      (if (not (Networking|IsDedicatedServer))
        ;;[1 1 1] If local controlled; init once..
        (Utilities|IsLocallyControlled :!label _label
          (:LocalControl
            (CallFunction|NotifyOwnerOfInstantiation)
            (if (not (Variables|Initialisation|GetInitialised))
              (Variables|Initialisation|SetInitialised true)
              ;;[1 1 1] Reload settings
              (CallFunction|CreateandShowToolsAssistInformation)
              (CallFunction|InitSettings)
              ;;[1 1 1] Create ghost light
              (CallFunction|CreateSelectionTarget "/Game/CustomContent/UGC2281370083/Blueprints/Rope/Props/RopeSelectionPointPropBP"))))))
    (:Remote
      (goto _label))))

(event EventTick
  (params (DeltaSeconds :type Float%20%28single-precision%29))
  ;[1 1 1] EVENT TICK
  (|CallParentFunction DeltaSeconds)
  (Utilities|IsLocallyControlled
    (:LocalControl
      (Networking|SwitchHasAuthority
        (:Authority
          ;;[1 1 1] Listen server?
          (if (not (Networking|IsDedicatedServer))
            ;;[1 1 1] Handle MOUSE SELECTION POINT
            (bind _returnvalue (Class|KJModToolProxy|GetPawnCameraComponent :!label _label))
            (bind (_outhit _returnvalue_2) (Collision|LineTraceByChannel (Transformation|GetWorldLocation _returnvalue) (+ (Transformation|GetWorldLocation _returnvalue) (* (Math|Vector|GetForwardVector _returnvalue) 3.5e+03)) "TraceTypeQuery1" true (Utilities|Array|MakeArray (Game|Player|GetPlayerPawn 0)) "None"))
            (if _returnvalue_2
              (Utilities|IsValid (.HitActor (Collision|BreakHitResult _outhit))
                (:Is%20Valid
                  (Utilities|IsValid (Variables|Targeting|GetSelectionTargetPointerActor) ; May not be replicated from server (yet)
                    (:Is%20Valid
                      (bind _rotation (Utilities|BuildRotationfromImpactNormal (.ImpactPoint (Collision|BreakHitResult _outhit)) (.ImpactNormal (Collision|BreakHitResult _outhit)))
                        (:Out
                          (Variables|Targeting|SetSelectionTargetLocation (.Location (Collision|BreakHitResult _outhit)))
                          (Variables|Targeting|SetSelectedTargetRotation _rotation)
                          (Variables|Targeting|SetSelectedActor (.HitActor (Collision|BreakHitResult _outhit)))
                          (CallFunction|SetRopeTargetOwningClient (Variables|Targeting|GetSelectionTargetLocation) true (Variables|Targeting|GetSelectedTargetRotation))
                          (Variables|Targeting|SetTargetIsViable true))))
                    (:Is%20Not%20Valid
                      (CallFunction|SetRopeTargetOwningClient "0, 0, 0" false "0, 0, 0" :!label _label_2)
                      (Variables|Targeting|SetTargetIsViable false))))
                (:Is%20Not%20Valid
                  (goto _label_2)))
              (else
                (goto _label_2)))))
        (:Remote
          (goto _label))))))

(event Custom|SpawnRopeServer
  (params (SourceConnectionActor :type Actor%20Object%20Reference) (DestinationConnectionActor :type Actor%20Object%20Reference) (SourceAnchorPoint :type Vector) (DestinationAnchorPoint :type Vector))
  (bind _settings (Variables|ToolSetting|GetSettings))
  (bind (_segments _colour _type _disablecollision _showjoints) (Utilities|Struct|BreakRopeToolActorSettings _settings))
  ;[1 1 1] Spawn Rope
  (bind _returnvalue (Game|SpawnActorfromClass "/Game/CustomContent/UGC2281370083/Blueprints/Rope/Visualisation/BuildARopeBP.BuildARopeBP_C" (Transformation|GetActorTransform) "Undefined" (Components|GetOwner) (Math|Float|Truncate _segments) SourceConnectionActor DestinationConnectionActor SourceAnchorPoint DestinationAnchorPoint _type _colour _showjoints _disablecollision 0))
  (Variables|Spawning|SetSpawnedRopeBuilderActor _returnvalue) ; Owner will get this, and update history
)

(event Custom|SpawnRopeOwningClient
  (params (SourceConnectionActor :type Actor%20Object%20Reference) (DestinationConnectionActor :type Actor%20Object%20Reference) (SourceAnchorPoint :type Vector) (DestinationAnchorPoint :type Vector))
  ;[1 1 1] Spawn Rope
  (CallFunction|SpawnRopeServer SourceConnectionActor DestinationConnectionActor SourceAnchorPoint DestinationAnchorPoint))

(event EventToolProxyItemSpawned
  (params (spawnedActor :type Actor%20Object%20Reference))
  ;[1 1 1] (interface) Item Spawned - From Pawn
  (bind _asrope_selection_point_prop_bp (Utilities|Casting|CastToRopeSelectionPointPropBP spawnedActor)
    (:then
      (Utilities|IsValid (Variables|Targeting|GetSelectionTargetPointerActor) ; First time? it's our "ghost" light
        (:Is%20Not%20Valid
          (Variables|Targeting|SetSelectionTargetPointerActor _asrope_selection_point_prop_bp))))
    (:CastFailed
      (|CallParentFunction spawnedActor) ; Probably a Q menu spawning; let parent deal with it
    )))

(event Custom|FlashBeam
  ;[1 1 1] FLASH BEAM
  (Networking|SwitchHasAuthority
    (:Authority
      ;;[1 1 1] Listen server?
      (if (not (Networking|IsDedicatedServer))
        (Rendering|SetVisibility (Variables|Default|GetParticleSystem) true false :!label _label)
        (Utilities|FlowControl|Delay 0.2)
        (Rendering|SetVisibility (Variables|Default|GetParticleSystem) false false)))
    (:Remote
      (goto _label))))

(event EventToolProxyPrimaryMouseClick
  (params (pressed :type Boolean))
  ;[1 1 1] LEFT/RIGHT MOUSE - Drop or freeze if anything on tool
  (if pressed ; Pressed?
    (Utilities|IsValid (Variables|Targeting|GetSelectionTargetPointerActor)
      (:Is%20Valid
        (if (<= (Variables|Default|GetRespawnDelayTimeout) 0.0)
          (if (Variables|Targeting|GetTargetIsViable)
            (Utilities|IsValid (Variables|Targeting|GetSelectedActor)
              (:Is%20Valid
                (CallFunction|FlashBeam)
                (bind _bhaslocalownership (Class|KJModOwnershipComponent|HasOwnershipRights 0 true (Utilities|GetPlayerSteamID) (Variables|Targeting|GetSelectedActor)))
                (if _bhaslocalownership
                  (if (Variables|Targeting|GetPrimaryTargetSelection)
                    (Variables|RopeBuilding|SetPrimaryTargetActor (Variables|Targeting|GetSelectedActor))
                    (Variables|RopeBuilding|SetPrimaryTargetLocation (Variables|Targeting|GetSelectionTargetLocation))
                    (Variables|Targeting|SetPrimaryTargetSelection false)
                    (Class|KJModToolProxy|ShowMessage "Rope source point selected" 2.0 true 0)
                    (Class|KJModToolProxy|PlayToolSoundEffect "ToolSelectionSound" true)
                    (elif (!= (Variables|RopeBuilding|GetPrimaryTargetActor) (Variables|Targeting|GetSelectedActor))
                      (CallFunction|SpawnRopeOwningClient (Variables|RopeBuilding|GetPrimaryTargetActor) (Variables|Targeting|GetSelectedActor) (Variables|RopeBuilding|GetPrimaryTargetLocation) (Variables|Targeting|GetSelectionTargetLocation))
                      (Variables|RopeBuilding|SetPrimaryTargetActor 0)
                      (Variables|Targeting|SetPrimaryTargetSelection true) ; Enable next clip to set primary (start again)
                      (Variables|Default|SetRespawnDelayTimeout 0.5)
                      (Class|KJModToolProxy|ShowMessage "Rope created!" 2.0 true 0)
                      (Class|KJModToolProxy|PlayToolSoundEffect "ToolSpawnSound" true)
                      (else
                        (Class|KJModToolProxy|ShowMessage "Source and destination must be different; rope creation cancelled" 2.0 true "/Game/CustomContent/UGC2281370083/Blueprints/Rope/Textures/RopeFailure.RopeFailure")
                        (Class|KJModToolProxy|PlayToolSoundEffect "ToolIllegalOpSound" true)
                        (Variables|Targeting|SetPrimaryTargetSelection true) ; Enable next clip to set primary (start again)
                      )))
                  (else
                    (CallFunction|ShowMessagetoLocalPlayer "You do not own the prop your trying to attach a rope to" 2.0 false)
                    (Variables|Targeting|SetPrimaryTargetSelection true) ; Enable next clip to set primary (start again)
                  ))))))))))

(event Custom|Setting_SetColor
  (params (Color :type Linear%20Color%20Structure))
  ;[1 1 1] Settings (from widgets and onload)
  (Utilities|Struct|SetmembersinRopeToolActorSettings (Variables|ToolSetting|GetSettings) Color)
  ;[1 1 1] Update server
  (if (Variables|ToolSetting|GetbServerSettingsInited)
    (CallFunction|SetLightSettingsOwningClient (Variables|ToolSetting|GetSettings))))

(event Custom|Setting_EnableShowJoints
  (params (Enabled :type Boolean))
  ;[1 1 1] Settings (from widgets and onload)
  (Utilities|Struct|SetmembersinRopeToolActorSettings (Variables|ToolSetting|GetSettings) Enabled)
  ;[1 1 1] Update server
  (if (Variables|ToolSetting|GetbServerSettingsInited)
    (CallFunction|SetLightSettingsOwningClient (Variables|ToolSetting|GetSettings))))

(event Custom|Setting_SetSegments
  (params (Value :type Float%20%28single-precision%29))
  ;[1 1 1] Settings (from widgets and onload)
  (Utilities|Struct|SetmembersinRopeToolActorSettings (Variables|ToolSetting|GetSettings) Value)
  ;[1 1 1] Update server
  (if (Variables|ToolSetting|GetbServerSettingsInited)
    (CallFunction|SetLightSettingsOwningClient (Variables|ToolSetting|GetSettings))))

(event Custom|Setting_DisableCollision
  (params (DisableCollision :type Boolean))
  ;[1 1 1] Settings (from widgets and onload)
  (Utilities|Struct|SetmembersinRopeToolActorSettings (Variables|ToolSetting|GetSettings) DisableCollision)
  ;[1 1 1] Update server
  (if (Variables|ToolSetting|GetbServerSettingsInited)
    (CallFunction|SetLightSettingsOwningClient (Variables|ToolSetting|GetSettings))))

(event Custom|SetLightSettingsOwningClient
  (params (Settings :type Rope%20Tool%20Actor%20Settings%20Structure))
  ;[1 1 1] Replicate changes (and visualise mesh)
  (CallFunction|SetLightSettingsServer Settings))

(event Custom|Setting_SetType
  (params (Type :type String))
  ;[1 1 1] Settings (from widgets and onload)
  (Utilities|Struct|SetmembersinRopeToolActorSettings (Variables|ToolSetting|GetSettings) Type)
  ;[1 1 1] Update server
  (if (Variables|ToolSetting|GetbServerSettingsInited)
    (CallFunction|SetLightSettingsOwningClient (Variables|ToolSetting|GetSettings))))

(event Custom|SetLightSettingsServer
  (params (Settings :type Rope%20Tool%20Actor%20Settings%20Structure))
  ;[1 1 1] Replicate changes (and visualise mesh)
  (Variables|ToolSetting|SetSettings Settings))

(event Custom|InitSettings
  ;[1 1 1] Init / Load previous settings
  (bind _returnvalue (Class|KJModToolProxy|LoadToolSettings "RopeToolSettings"))
  (Utilities|IsValid _returnvalue ; No save? use defaults
    (:Is%20Valid
      (bind _asrope_tool_save_game_bp (Utilities|Casting|CastToRopeToolSaveGameBP _returnvalue))
      (Utilities|FlowControl|Sequence
        (:then_0
          ;[1 1 1] Local Initial settings
          (Utilities|FlowControl|Sequence
            (:then_0
              (CallFunction|SettingSetSegments (Variables|/Game/CustomContent/UGC2281370083/Blueprints/Rope/RopeToolSaveGameBP.RopeToolSaveGameBP_C|GetSegments _asrope_tool_save_game_bp)))
            (:then_1
              (CallFunction|SettingSetColor (Variables|/Game/CustomContent/UGC2281370083/Blueprints/Rope/RopeToolSaveGameBP.RopeToolSaveGameBP_C|GetColor _asrope_tool_save_game_bp)))
            (:then_3
              (CallFunction|SettingSetType (Variables|/Game/CustomContent/UGC2281370083/Blueprints/Rope/RopeToolSaveGameBP.RopeToolSaveGameBP_C|GetType _asrope_tool_save_game_bp)))
            (:then_4
              (CallFunction|SettingDisableCollision (Variables|/Game/CustomContent/UGC2281370083/Blueprints/Rope/RopeToolSaveGameBP.RopeToolSaveGameBP_C|GetbDisableCollision _asrope_tool_save_game_bp)))
            (:then_5
              (CallFunction|SettingEnableShowJoints (Variables|/Game/CustomContent/UGC2281370083/Blueprints/Rope/RopeToolSaveGameBP.RopeToolSaveGameBP_C|GetbShowJoints _asrope_tool_save_game_bp)))))
        (:then_1
          ;[1 1 1] Init settings server
          (CallFunction|SetLightSettingsOwningClient (Variables|ToolSetting|GetSettings) :!label _label)
          (Variables|ToolSetting|SetbServerSettingsInited true))))
    (:Is%20Not%20Valid
      (goto _label))))

(fn ConstructionScript)

(fn CreateandShowToolsAssistInformation
  (Class|KJModToolProxy|ShowToolAssistUI)
  (Class|KJModToolProxy|SetToolAssistTitle "Rope" "A rope that can join together physics objects")
  (Class|KJModToolProxy|ClearToolAssistFunctions)
  (bind _returnvalue (Class|KJModToolProxy|CreateToolAssistFunction "Add rope at required point"))
  (Class|KJModToolProxy|SetToolAssistFunctionPrimaryDetails _returnvalue "LeftMouse"))

(fn CreateSelectionTarget
  (params (AssetPath :type String))
  (bind _returnvalue (Game|GetPlayerCameraManager 0))
  (Class|KJModToolProxy|SpawnItem AssetPath (+ (Transformation|GetActorLocation _returnvalue) (* (Transformation|GetActorForwardVector _returnvalue) 5e+02)) "0, 0, 0" "1.000000,1.000000,1.000000"))

(fn ToolProxyGetToolSettingPanel
  (Utilities|IsValid (Variables|ToolSetting|GetToolSettingsWidget)
    (:Is%20Valid
      _)
    (:Is%20Not%20Valid
      (bind _returnvalue (UserInterface|CreateWidget "/Game/CustomContent/UGC2281370083/Blueprints/Rope/Settings/RopeToolSettingsWidgetBP.RopeToolSettingsWidgetBP_C" (Game|GetPlayerController 0) self))
      (Default|CreatedEvent _returnvalue)
      (Variables|ToolSetting|SetToolSettingsWidget _returnvalue)))
  (return (Variables|ToolSetting|GetToolSettingsWidget)))

(fn OnRepSpawnedRopeBuilderActor
  (bind _spawnedropebuilderactor (Variables|Spawning|GetSpawnedRopeBuilderActor))
  ;[1 1 1] If we're the owner then record the rope creation in our history (for delete)
  (Utilities|IsLocallyControlled
    (:LocalControl
      (Utilities|IsValid _spawnedropebuilderactor
        (:Is%20Valid
          (CallFunction|UpdateHistoryOwningClient _spawnedropebuilderactor))))))