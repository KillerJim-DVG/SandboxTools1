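; RopeVisualiserBP is a custom-content actor that draws a rope through an array of attach-point actors.
; On BeginPlay it retries every 0.1 seconds until all points are valid, allowing for replication, then adds a KJModRopeComponent.
; Clients apply a dynamic cord material using the Pak texture named by MaterialType and a colour.
; Material tiling scales with first-to-last point distance, and the last FakeRopeSectionBP's EndPoint becomes the rope's start component.
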(event EventBeginPlay
  (Development|PrintString (Utilities|String|Append "RopeVIsualiderBP Called, mat: " (Variables|Default|GetMaterialType)) true true "(R=1.000000,G=0.000000,B=0.041492,A=1.000000)" 22.0)
  ;[1 1 1] Make sure everything is replicated
  (bind _valid (CallFunction|AreActorsValid :!label _label))
  (if _valid
    ;[1 1 1] Make the rope visualiser
    (bind _returnvalue (AddComponent|AddKJModRopeComponent false))
    (Utilities|HandleClientServerLogic
      (:ServerLogic
        _)
      (:ClientLogic
        (bind _returnvalue_2 (Class|KJModProxy|GetPakFileObject (Variables|Default|GetMaterialType)))
        (bind _astexture_2d (Utilities|Casting|CastToTexture2D _returnvalue_2)
          (:then
            (bind _returnvalue_3 (Rendering|Material|CreateDynamicMaterialInstance "/Game/CustomContent/UGC2281370083/Blueprints/Rope/Textures/RopeCordMat.RopeCordMat" "None" :!class /Script/Engine.KismetMaterialLibrary))
            (Rendering|Material|SetTextureParameterValue _returnvalue_3 "TextureParam" _astexture_2d)
            (Rendering|Material|SetVectorParameterValue _returnvalue_3 "ColorParam" (Variables|Default|GetColor) :!class /Script/Engine.MaterialInstanceDynamic)
            (Rendering|Material|SetMaterial _returnvalue 0 _returnvalue_3))
          (:CastFailed
            _))))
    ;[1 1 1] First point needs to have the start component set; this allows it section of rope to reach back to the origin
    (Variables|/Script/KillerJimModProxy.KJModRopeComponent|SetAttachPoints _returnvalue (Variables|Default|GetAttachPoints))
    (bind _value (CallFunction|CalcDistance))
    (Variables|/Script/KillerJimModProxy.KJModRopeComponent|SetTileMaterial _returnvalue (/ _value 1e+01))
    (bind _asfake_rope_section_bp (Utilities|Casting|CastToFakeRopeSectionBP (Utilities|Array|Get(acopy) (Variables|Default|GetAttachPoints) (- (Utilities|Array|Length (Variables|Default|GetAttachPoints)) 1))))
    (Variables|/Script/KillerJimModProxy.KJModRopeComponent|SetStartPointComponent _returnvalue (Variables|/Game/CustomContent/UGC2281370083/Blueprints/Rope/Visualisation/FakeRopeSectionBP.FakeRopeSectionBP_C|GetEndPoint _asfake_rope_section_bp))
    (else
      (Utilities|FlowControl|Delay 0.1)
      (goto _label))))

(fn ConstructionScript)

(fn AreActorsValid
  (for _array_element (Variables|Default|GetAttachPoints)
    (if (== _array_element 0)
      (return false)))
  (return true))

(fn CalcDistance
  (bind _attachpoints (Variables|Default|GetAttachPoints))
  (return (Transformation|GetDistanceTo (Utilities|Array|Get(acopy) _attachpoints) (Utilities|Array|Get(acopy) (Variables|Default|GetAttachPoints) (- (Utilities|Array|Length _attachpoints) 1)))))