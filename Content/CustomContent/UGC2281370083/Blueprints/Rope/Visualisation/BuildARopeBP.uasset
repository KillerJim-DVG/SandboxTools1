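; Builds a physics-driven rope between source and destination anchor points and attaches it to the two connection actors.
; On authority, BuildRope spawns a chain of scaled FakeRopeSectionBP segments joined by replicated physics constraint actors, plus a joint at each end.
; SpawnClientRopeVisualisation polls until the segment references replicate, then spawns a RopeVisualiserBP over them for client display.
; Destroying the actor removes the visualiser, segments and tracked constraints.
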(event Custom|SpawnClientRopeVisualisation
  (params (RopeInstantiation :type Rope%20Instantiation%20Struct%20Structure))
  (bind _materialtype (Variables|Default|GetMaterialType))
  ;[1 1 1] Visualise the rope on clients
  ;;[1 1 1] Wait until everything is replicated
  (bind _valid (CallFunction|IsRopeStructReplicated :!label _label))
  (if _valid
    (Development|PrintString _materialtype true true "(R=1.000000,G=0.000000,B=0.041492,A=1.000000)" 22.0)
    (bind _returnvalue (Game|SpawnActorfromClass "/Game/CustomContent/UGC2281370083/Blueprints/Rope/Visualisation/RopeVisualiserBP.RopeVisualiserBP_C" (Transformation|GetActorTransform) "AlwaysSpawn" self (Utilities|Struct|BreakRopeInstantiationStruct RopeInstantiation) _materialtype (Variables|Default|GetColor) 0)) ; Replicated actir
    (Variables|Default|SetSpawnedRopeVisualiser _returnvalue)
    (else
      (Utilities|FlowControl|Delay 0.1)
      (goto _label))))

(event EventBeginPlay
  ;[1 1 1] BEGIN PLAY - Calculate some maths for the rope segments moving from src to dst
  (Variables|Default|SetDirectionalVector (Math|Vector|Normalize (- (Variables|Default|GetDestinationAnchorPoint) (Variables|Default|GetSourceAnchorPoint))))
  (Variables|Default|SetSegmentLength (/ (Math|Vector|Distance(Vector) (Variables|Default|GetSourceAnchorPoint) (Variables|Default|GetDestinationAnchorPoint)) (Math|Conversions|ToFloat(Integer) (+ (Variables|Default|GetSegmentCount) 1))))
  (CallFunction|BuildRope))

(event EventDestroyed
  ;[1 1 1] DESTROY - Remove everything, only the rope visualiser is valid on the client (both both c/s run this code)
  (Utilities|IsValid (Variables|Default|GetSpawnedRopeVisualiser)
    (:Is%20Valid
      (Actor|DestroyActor (Variables|Default|GetSpawnedRopeVisualiser)))
    (:Is%20Not%20Valid
      _))
  (for _array_element (Variables|Default|GetSpawnSegmentActors)
    (Utilities|IsValid _array_element
      (:Is%20Valid
        (Actor|DestroyActor _array_element))))
  (for _array_element_2 (Variables|Default|GetSpawnPhysicsActors)
    (Utilities|IsValid _array_element_2
      (:Is%20Valid
        (Actor|DestroyActor _array_element_2)))))

(fn ConstructionScript)

(fn BuildRope
  (bind _attachedactors (LocalVariables|GetAttachedActors))
  (bind _attachedactors_2 (LocalVariables|GetAttachedActors))
  (bind _returnvalue (Utilities|Array|Length _attachedactors_2))
  (bind _output (Utilities|Array|Get(acopy) _attachedactors))
  (bind _returnvalue_2 (- _returnvalue 1))
  (bind _output_2 (Utilities|Array|Get(acopy) _attachedactors_2 _returnvalue_2))
  (Networking|SwitchHasAuthority
    (:Authority
      (for _index (range 0 (Variables|Default|GetSegmentCount))
        (bind _outputpin (CallFunction|SpawnMesh (Math|Transform|MakeTransform (+ (Variables|Default|GetSourceAnchorPoint) (LocalVariables|GetSegmentOffset)) (Math|Rotator|MakeRotfromZ (Variables|Default|GetDirectionalVector)) (Math|Vector|MakeVector 1.0 1.0 (/ (Variables|Default|GetSegmentLength) 105.0)))))
        (Utilities|Array|Add (LocalVariables|GetAttachedActors) _outputpin)
        (bind _output_get (LocalVariables|SetSegmentOffset (+ (LocalVariables|GetSegmentOffset) (* (Variables|Default|GetDirectionalVector) (Variables|Default|GetSegmentLength)))))
        (LocalVariables|SetSpawnTransform (Math|Transform|MakeTransform (+ (Variables|Default|GetSourceAnchorPoint) _output_get) (Math|Rotator|MakeRotfromZ (Variables|Default|GetDirectionalVector))))
        (Utilities|IsValid (LocalVariables|GetPreviousPhysicsActor)
          (:Is%20Valid
            (Class|PhysicsConstraintComponent|SetConstrainedComponents (Variables|/Script/Engine.PhysicsConstraintActor|GetConstraintComp (LocalVariables|GetPreviousPhysicsActor)) (Actor|GetComponentbyClass (LocalVariables|GetPreviousMeshActor) "/Script/Engine.PrimitiveComponent") "None" (Actor|GetComponentbyClass _outputpin "/Script/Engine.PrimitiveComponent") "None")
            (Class|PhysicsConstraintComponent|SetDisableCollision (Variables|/Script/Engine.PhysicsConstraintActor|GetConstraintComp (LocalVariables|GetPreviousPhysicsActor)) true)
            (LocalVariables|SetPreviousMeshActor _outputpin)
            (bind _outputpin_2 (CallFunction|SpawnPhysicsContraint (LocalVariables|GetSpawnTransform)))
            (bind _output_get_2 (LocalVariables|SetPreviousPhysicsActor _outputpin_2))
            (Utilities|Array|Add (LocalVariables|GetAttachedPhysicsActors) _output_get_2))
          (:Is%20Not%20Valid
            (bind _outputpin_3 (CallFunction|SpawnPhysicsContraint (LocalVariables|GetSpawnTransform)))
            (bind _output_get_3 (LocalVariables|SetPreviousPhysicsActor _outputpin_3))
            (Utilities|Array|Add (LocalVariables|GetAttachedPhysicsActors) _output_get_3)
            (LocalVariables|SetPreviousMeshActor _outputpin))))
      ;[1 1 1] Get client to make rope visualisation
      (CallFunction|SpawnClientRopeVisualisation (Utilities|Struct|MakeRopeInstantiationStruct (LocalVariables|GetAttachedActors)))
      ;[1 1 1] Pass "up" the arrays from local versions to the actors
      (Variables|Default|SetSpawnSegmentActors (LocalVariables|GetAttachedActors))
      (Variables|Default|SetSpawnPhysicsActors (LocalVariables|GetAttachedPhysicsActors))
      ;[1 1 1] Source Joint
      (Utilities|FlowControl|Sequence
        (:then_0
          (bind _outputpin_4 (CallFunction|SpawnPhysicsContraint (Transformation|GetActorTransform _output)))
          (Class|PhysicsConstraintComponent|SetConstrainedComponents (Variables|/Script/Engine.PhysicsConstraintActor|GetConstraintComp _outputpin_4) (Actor|GetComponentbyClass _output "/Script/Engine.PrimitiveComponent") "None" (Actor|GetComponentbyClass (Variables|Default|GetSourceConnectionActor) "/Script/Engine.PrimitiveComponent") "None")
          (Class|PhysicsConstraintComponent|SetDisableCollision (Variables|/Script/Engine.PhysicsConstraintActor|GetConstraintComp _outputpin_4) true))
        (:then_1
          ;[1 1 1] Source Joint
          (bind _outputpin_5 (CallFunction|SpawnPhysicsContraint (Transformation|GetWorldTransform (Variables|/Game/CustomContent/UGC2281370083/Blueprints/Rope/Visualisation/FakeRopeSectionBP.FakeRopeSectionBP_C|GetEndSphere _output_2))))
          (Class|PhysicsConstraintComponent|SetConstrainedComponents (Variables|/Script/Engine.PhysicsConstraintActor|GetConstraintComp _outputpin_5) (Actor|GetComponentbyClass _output_2 "/Script/Engine.PrimitiveComponent") "None" (Actor|GetComponentbyClass (Variables|Default|GetDestinationConnectionActor) "/Script/Engine.PrimitiveComponent") "None")
          (Class|PhysicsConstraintComponent|SetDisableCollision (Variables|/Script/Engine.PhysicsConstraintActor|GetConstraintComp _outputpin_5) true))))))

(fn SpawnMesh
  (params (SpawnTransform :type Transform))
  (bind _returnvalue (Game|SpawnActorfromClass "/Game/CustomContent/UGC2281370083/Blueprints/Rope/Visualisation/FakeRopeSectionBP.FakeRopeSectionBP_C" SpawnTransform "AlwaysSpawn" self (Variables|Default|GetbDisableCollision) (Variables|Default|GetbShowJoints) 0))
  (return _returnvalue))

(fn SpawnPhysicsContraint
  (params (SpawnTransform :type Transform))
  ;[1 1 1] Spawn and replicate the physics contraint between rope segments
  (bind _returnvalue (Game|SpawnActorfromClass "/Script/Engine.PhysicsConstraintActor" SpawnTransform "AlwaysSpawn" self 0))
  (Networking|SetReplicates _returnvalue true)
  (Class|Actor|SetReplicateMovement _returnvalue true)
  (Variables|/Script/Engine.Actor|SetbAlwaysRelevant _returnvalue true)
  (Variables|/Script/Engine.Actor|SetbAlwaysRelevant _returnvalue true)
  (Class|ActorComponent|SetIsReplicated (Variables|/Script/Engine.PhysicsConstraintActor|GetConstraintComp _returnvalue) true)
  (Class|PhysicsConstraintComponent|SetLinearZLimit (Variables|/Script/Engine.PhysicsConstraintActor|GetConstraintComp _returnvalue) "LCM_Locked" 15.0)
  (return _returnvalue))

(fn IsRopeStructReplicated
  (for _array_element (Utilities|Struct|BreakRopeInstantiationStruct (Variables|Default|GetRopeInstantiationStruct))
    (if (== _array_element 0)
      (return false)))
  (return true))